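; AC_Inventory is an inventory component that stores captured enemy ingredients and handles the player's interact trace.
; AddIngredient saves ingredient type, perfection level and skeletal mesh in an incrementing-key map, intended for spawning objects later.
; On BeginPlay it binds Interact to the first-person character's input event.
; Interact line-traces on the Camera channel from above the owner along the camera rotation, with debug drawing, and sends an interact message to the hit actor.
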(event `AddIngredient`
  (params (Ingredient :type "/Game/Scripting/Blueprints/Enemys/Enums/E_IngredientType Enum" :default "NewEnumerator0") (PerfectionLevel :type "/Game/Scripting/Blueprints/Enemys/Health/E_PerfectionLevel Enum" :default "NewEnumerator4") (SkeletalMesh :type "SkeletalMesh Object Reference"))
  (bind _capturekey (`self.CaptureKey`))
  ;[0.5 0.7 1] Adds Stats to Map, will be stored and then the objects can be spawned later on with this information
  (`BlueprintMapLibrary.Map_Add` (`self.CapturedIngredients`) _capturekey (make `/Game/Scripting/Blueprints/Character/F_CapturedEnemyStats` Ingredient PerfectionLevel SkeletalMesh))
  (bind _result (`/Engine/EditorBlueprintResources/StandardMacros.IncrementInt` _capturekey)
    (:`  `
      (`KismetSystemLibrary.PrintText` (`KismetTextLibrary.Conv_IntToText` _result)))))

(event `self.ReceiveBeginPlay`
  ;[0.5 0.7 1] Set up bind to input event (This code can be moved to first person character) Perform a line trace and activate interact in whatever is traced
  (bind _returnvalue (`GameplayStatics.GetActorOfClass` "/Game/Scripting/Blueprints/Character/BP_FirstPersonCharacter.BP_FirstPersonCharacter_C"))
  (add `/Game/Scripting/Blueprints/Character/BP_FirstPersonCharacter.OnInput` _returnvalue (delegate `Interact`)))

(event `Interact`
  (bind _returnvalue (+ (`Actor.K2_GetActorLocation` (`self.GetOwner`)) (0.0 0.0 60.0)))
  ;[0.5 0.7 1] Set up bind to input event (This code can be moved to first person character) Perform a line trace and activate interact in whatever is traced
  (bind _outhit (`KismetSystemLibrary.LineTraceSingle` :`Start` _returnvalue :`End` (+ _returnvalue (* (`PlayerCameraManager.GetCameraRotation` (`GameplayStatics.GetPlayerCameraManager` 0)) (`self.InteractDistance`))) :`TraceChannel` "TraceTypeQuery2" :`DrawDebugType` "ForDuration"))
  (message `/Game/Scripting/Blueprints/ConveyorBelt/BPI_Interact.Interact` (`.HitActor` (`GameplayStatics.BreakHitResult` _outhit))))