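; Actor component that switches the first-person character between five weapons: flamethrower, cloche gun, seasoning shotgun, sauce gun and knife.
; It binds to the character's direct-select and scroll events, with scrolling wrapping around and briefly locked by a timer.
; Each swap changes the weapon's child actor class and the first-person mesh, anim class and transform.
; It then reattaches the weapon to its socket and broadcasts the matching enum through OnWeaponSwap.
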(event `self.ReceiveBeginPlay`
  (bind _first_person_character_reference (`self.First Person Character Reference`))
  ;[1 0.7219 0] Initialise and bind events
  (bind _asbp_first_person_character (cast `/Game/Scripting/Blueprints/Character/BP_FirstPersonCharacter` (`self.GetOwner`))
    (:`then`
      (set `self.First Person Character Reference` _asbp_first_person_character)
      (add `/Game/Scripting/Blueprints/Character/BP_FirstPersonCharacter.OnSwapWeapon1` _first_person_character_reference (`|CreateDelegate` :!event `Weapon1`))
      (add `/Game/Scripting/Blueprints/Character/BP_FirstPersonCharacter.OnSwapWeapon2` _first_person_character_reference (`|CreateDelegate` :!event `Weapon2`))
      (add `/Game/Scripting/Blueprints/Character/BP_FirstPersonCharacter.OnSwapWeapon3` _first_person_character_reference (`|CreateDelegate` :!event `Weapon3`))
      (add `/Game/Scripting/Blueprints/Character/BP_FirstPersonCharacter.OnSwapWeapon4` _first_person_character_reference (`|CreateDelegate` :!event `Weapon4`))
      (add `/Game/Scripting/Blueprints/Character/BP_FirstPersonCharacter.OnSwapWeapon5` _first_person_character_reference (`|CreateDelegate` :!event `Weapon5`))
      (add `/Game/Scripting/Blueprints/Character/BP_FirstPersonCharacter.OnScrollUp` _first_person_character_reference (`|CreateDelegate` :!event `ScrollUp`))
      (add `/Game/Scripting/Blueprints/Character/BP_FirstPersonCharacter.OnScrollDown` _first_person_character_reference (`|CreateDelegate` :!event `ScrollDown`))
      (set `self.First Person Mesh` (`/Game/Scripting/Blueprints/Character/BP_FirstPersonCharacter.FirstPersonMesh` (`self.First Person Character Reference`))))
    (:`CastFailed`
      (`KismetSystemLibrary.PrintString` "AC_WeaponSwapping: Cast to FP Character failed" true true (struct :`R` 1.0 :`A` 1.0) 10.0))))

(event `VisualChange/LocationSetup`
  (bind _first_person_character_reference (`self.First Person Character Reference`))
  (bind _firstpersonmesh (`/Game/Scripting/Blueprints/Character/BP_FirstPersonCharacter.FirstPersonMesh` (`self.First Person Character Reference`)))
  (bind _bp_weapon_parent (`/Game/Scripting/Blueprints/Character/BP_FirstPersonCharacter.BP_Weapon_Parent` _first_person_character_reference))
  ;[1 0.7892 0] Actually change values
  (`|ExecutionSequence`
    (:`then_0`
      (`SkinnedMeshComponent.SetSkinnedAssetAndUpdate` _firstpersonmesh (`self.New Mesh`) true))
    (:`then_1`
      (`SkeletalMeshComponent.SetAnimInstanceClass` _firstpersonmesh (`self.New Anim Instance Class`)))
    (:`then_2`
      (`SceneComponent.K2_SetRelativeLocationAndRotation` _firstpersonmesh (`self.New Location`) (`self.New Rotation`) false false))
    (:`then_3`
      (`SceneComponent.K2_DetachFromComponent` _bp_weapon_parent "KeepRelative" "KeepRelative" "KeepRelative" true)
      (`SceneComponent.K2_AttachToComponent` _bp_weapon_parent (`/Game/Scripting/Blueprints/Character/BP_FirstPersonCharacter.FirstPersonMesh` _first_person_character_reference) (`self.Socket Name`) "KeepRelative" "SnapToTarget" "SnapToTarget" true)
      ;[0.1927 0 0] PassEnumToPlayer
      (`self.OnWeaponSwap` (`BlueprintMapLibrary.Map_Find` (`self.Class-EnumMap`) (`self.CurrentWeaponClass`))))))

(event `Weapon1`
  ;[1 0.7892 0] Button Weapon swap
  (set `self.Current Weapon` 0)
  ;[0.1927 0 0] Set weapon class
  (bind _output_get (set `self.CurrentWeaponClass` "/Game/Scripting/Blueprints/Weapons/BP_FlamethrowerProt.BP_FlamethrowerProt_C" :!label _label))
  ;[1 0.7892 0] Set Child Actor
  (`ChildActorComponent.SetChildActorClass` (`/Game/Scripting/Blueprints/Character/BP_FirstPersonCharacter.BP_Weapon_Parent` (`self.First Person Character Reference`)) _output_get)
  ;[1 0.7892 0] Flamethrower
  (set `self.New Mesh` "/Game/Animation/Flamethrower/SK_Flamethrower.SK_Flamethrower")
  (set `self.New Anim Instance Class` "/Game/Animation/Flamethrower/ABP_Flamethrower.ABP_Flamethrower_C")
  (set `self.New Location` (10.0 10.0 -20.0))
  (set `self.New Rotation` (struct :`Yaw` -90.0))
  (set `self.Socket Name` "WeaponSocket")
  (`self.VisualChange/LocationSetup` :!label _label_2))

(event `Weapon2`
  ;[1 0.7892 0] Button Weapon swap
  (set `self.Current Weapon` 1)
  ;[0.1927 0 0] Set weapon class
  (bind _output_get (set `self.CurrentWeaponClass` "/Game/Scripting/Blueprints/Weapons/BP_FlyingSaucer.BP_FlyingSaucer_C" :!label _label_3))
  ;[1 0.7892 0] Set Child Actor
  (`ChildActorComponent.SetChildActorClass` (`/Game/Scripting/Blueprints/Character/BP_FirstPersonCharacter.BP_Weapon_Parent` (`self.First Person Character Reference`)) _output_get)
  ;[1 0.7892 0] ClocheGun
  (set `self.New Mesh` "/Game/Scripting/FirstPerson/FirstPersonArms/Character/Mesh/SK_Mannequin_Arms.SK_Mannequin_Arms")
  (set `self.New Anim Instance Class` "/Game/Scripting/FirstPerson/FirstPersonArms/Animations/FirstPerson_AnimBP.FirstPerson_AnimBP_C")
  (set `self.New Location` (3.0 -5.0 -161.0))
  (set `self.New Rotation` (struct :`Pitch` 1.92 :`Yaw` -19.9 :`Roll` 5.28))
  (set `self.Socket Name` "GripPoint")
  (goto _label_2))

(event `Swap`
  (bind _bp_weapon_parent (`/Game/Scripting/Blueprints/Character/BP_FirstPersonCharacter.BP_Weapon_Parent` (`self.First Person Character Reference`)))
  ;[1 0.7892 0] ForScrollWheel
  (switch `int` (`self.Current Weapon`)
    (:`0`
      (goto _label))
    (:`1`
      (goto _label_3))
    (:`2`
      ;[0.1927 0 0] Set weapon class
      (bind _output_get (set `self.CurrentWeaponClass` "/Game/Scripting/Blueprints/Weapons/BP_SeasoningGun.BP_SeasoningGun_C" :!label _label_4))
      ;[1 0.7892 0] Set Child Actor
      (`ChildActorComponent.SetChildActorClass` _bp_weapon_parent _output_get)
      ;[1 0.7892 0] SeasoningShotgun
      (set `self.New Mesh` "/Game/Animation/KnifeV2/SK_RiggedArms.SK_RiggedArms")
      (set `self.New Anim Instance Class` "/Game/Animation/KnifeV2/ABP_RiggedArmsV2.ABP_RiggedArmsV2_C")
      (set `self.New Location` (0.0 0.0 -170.0))
      (set `self.New Rotation` (struct :`Yaw` -90.0))
      (set `self.Socket Name` "GripPoint")
      (goto _label_2))
    (:`3`
      (bind _output_get_2 (set `self.CurrentWeaponClass` "/Game/Scripting/Blueprints/Weapons/BP_Sauce_Dispatcher.BP_Sauce_Dispatcher_C" :!label _label_5))
      (`ChildActorComponent.SetChildActorClass` _bp_weapon_parent _output_get_2)
      ;[1 0.7892 0] SauceGun
      (set `self.New Mesh` "/Game/Animation/KnifeV2/SK_RiggedArms.SK_RiggedArms")
      (set `self.New Anim Instance Class` "/Game/Animation/KnifeV2/ABP_RiggedArmsV2.ABP_RiggedArmsV2_C")
      (set `self.New Location` (0.0 -5.0 -170.0))
      (set `self.New Rotation` (struct :`Yaw` -90.0))
      (set `self.Socket Name` "GripPoint")
      (goto _label_2))
    (:`4`
      (bind _output_get_3 (set `self.CurrentWeaponClass` "/Game/Scripting/Blueprints/Weapons/BP_KnifeMelee.BP_KnifeMelee_C" :!label _label_6))
      (`ChildActorComponent.SetChildActorClass` (`/Game/Scripting/Blueprints/Character/BP_FirstPersonCharacter.BP_Weapon_Parent` (`self.First Person Character Reference`)) _output_get_3)
      ;[1 0.7892 0] Knife
      (set `self.New Mesh` "/Game/Animation/KnifeV2/SK_RiggedArms.SK_RiggedArms")
      (set `self.New Anim Instance Class` "/Game/Animation/KnifeV2/ABP_RiggedArmsV2.ABP_RiggedArmsV2_C")
      (set `self.New Location` (0.0 -5.0 -157.5))
      (set `self.New Rotation` (struct :`Yaw` -90.0))
      (set `self.Socket Name` "GripPoint")
      (goto _label_2))))

(event `Weapon3`
  ;[1 0.7892 0] Button Weapon swap
  (set `self.Current Weapon` 2)
  (goto _label_4))

(event `Weapon4`
  ;[1 0.7892 0] Button Weapon swap
  (set `self.Current Weapon` 3)
  (goto _label_5))

(event `Weapon5`
  ;[1 0.7892 0] Button Weapon swap
  (set `self.Current Weapon` 4)
  (goto _label_6))

(event `ScrollUp`
  (bind _current_weapon (`self.Current Weapon`))
  ;[1 0.7892 0] Scroll Wheel function
  (if (`self.CanSwap`)
    (set `self.CanSwap` false)
    (if (< _current_weapon 4)
      (`/Engine/EditorBlueprintResources/StandardMacros.IncrementInt` _current_weapon
        (:`  `
          _))
      (else
        (set `self.Current Weapon` 0)))
    (`self.Swap` :!label _label_7)
    (`KismetSystemLibrary.K2_SetTimerDelegate` (delegate `CustomEvent_0`) 0.05)))

(event `ScrollDown`
  (bind _current_weapon (`self.Current Weapon`))
  ;[1 0.7892 0] Scroll Wheel function
  (if (`self.CanSwap`)
    (set `self.CanSwap` false)
    (if (> _current_weapon 0)
      (`/Engine/EditorBlueprintResources/StandardMacros.DecrementInt` _current_weapon
        (:`  `
          (goto _label_7)))
      (else
        (set `self.Current Weapon` 4)
        (goto _label_7)))))

(event `CustomEvent_0`
  ;[1 0.7892 0] Scroll Wheel function
  (set `self.CanSwap` true))