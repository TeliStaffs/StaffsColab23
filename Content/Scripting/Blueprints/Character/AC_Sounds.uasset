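; AC_Sounds is a component that plays surface-dependent footstep sounds for the first-person player character.
; Each PlayPlayerFootstepsSFX call line-traces downward to pick the footstep cue from the physical surface type, then checks velocity for horizontal movement with zero vertical speed.
; Movement starts a looping timer, guarded by a DoOnce, that plays the cue below the actor; otherwise the timer clears.
; The PlayFootstepSound function is an empty stub.
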(event `self.ReceiveBeginPlay`
  ;[1 0 1] Get Player Refrence
  (bind _asbp_first_person_character (cast `/Game/Scripting/Blueprints/Character/BP_FirstPersonCharacter` (`GameplayStatics.GetPlayerCharacter` 0)))
  (set `self.playerRef` _asbp_first_person_character))

(event `PlayPlayerFootstepsSFX`
  (bind (_returnvalue_x _returnvalue_y _returnvalue_z) (`KismetMathLibrary.BreakVector` (`Actor.GetVelocity` (`self.playerRef`))))
  ;[1 0 1] Play Footsteps SFX
  (`self.CheckGroundMaterial`)
  (if (and (or (> _returnvalue_x 2.0) (< _returnvalue_x -2.0) (> _returnvalue_y 2.0) (< _returnvalue_y -2.0)) (== _returnvalue_z 0.0))
    (`/Engine/EditorBlueprintResources/StandardMacros.DoOnce` false :!label _label
      (:`Completed`
        (bind _returnvalue (`KismetSystemLibrary.K2_SetTimerDelegate` (delegate `PlayFootstepsSFX`) (`self.footstepInterval`) true))))
    (else
      (`KismetSystemLibrary.K2_ClearAndInvalidateTimerHandle` _returnvalue)
      (goto _label :!via `Reset`))))

(event `PlayFootstepsSFX`
  ;[1 0 1] Play Footsteps SFX
  (`GameplayStatics.PlaySoundAtLocation` (`self.footstepSFX`) (- (`Actor.K2_GetActorLocation` (`self.playerRef`)) (0.0 0.0 44.0)) (struct) 1.0 1.0 0.0 null null null null))

(event `CheckGroundMaterial`
  (bind _returnvalue (`Actor.K2_GetActorLocation` (`self.playerRef`)))
  ;[1 0 1] Play Footsteps SFX
  (bind (_outhit _returnvalue_2) (`KismetSystemLibrary.LineTraceSingle` _returnvalue (- _returnvalue (0.0 0.0 144.0)) "TraceTypeQuery1"))
  (if _returnvalue_2
    (switch `EPhysicalSurface` (`GameplayStatics.GetSurfaceType` _outhit)
      (:`SurfaceType_Default`
        (set `self.footstepSFX` "/Game/Audio/SoundEffects/Footsteps/SC_Default_Footstep.SC_Default_Footstep"))
      (:`SurfaceType1`
        (set `self.footstepSFX` "/Game/Audio/SoundEffects/Footsteps/SC_Dirt_Footstep.SC_Dirt_Footstep"))
      (:`SurfaceType2`
        (set `self.footstepSFX` "/Game/Audio/SoundEffects/Footsteps/SC_Grass_Footstep.SC_Grass_Footstep"))
      (:`SurfaceType3`
        (set `self.footstepSFX` "/Game/Audio/SoundEffects/Footsteps/SC_Stone_Footstep.SC_Stone_Footstep"))
      (:`SurfaceType4`
        (set `self.footstepSFX` "/Game/Audio/SoundEffects/Footsteps/SC_Water_Footstep.SC_Water_Footstep"))
      (:`SurfaceType5`
        (set `self.footstepSFX` "/Game/Audio/SoundEffects/Footsteps/SC_Wood_Footstep.SC_Wood_Footstep")))))

(fn `PlayFootstepSound`)