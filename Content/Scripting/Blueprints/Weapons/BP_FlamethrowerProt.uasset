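; Flamethrower weapon Blueprint that attaches to the first-person character on overlap and binds its fire, release and reload events.
; While firing, a looping timer spawns flame projectiles in a random cone along the camera, alongside particles, audio, camera shake and a glowing material.
; Each shot adds heat, shown through the ammo counter, and restarts a delayed timer-driven cooldown.
; Overheating or reloading plays a montage that blocks firing until it completes.
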(event `self.BeginPlayGuns`
  (bind _asbp_first_person_character (cast `/Game/Scripting/Blueprints/Character/BP_FirstPersonCharacter` (stale `self.SphereCollision.OnComponentBeginOverlap` OtherActor) :!label _label))
  (set `self.FirstPersonCharacterReference` _asbp_first_person_character)
  (`self.K2_AttachToComponent` self (`/Game/Scripting/Blueprints/Character/BP_FirstPersonCharacter.FirstPersonMesh` (`self.FirstPersonCharacterReference`)) "GripPoint" "SnapToTarget" "SnapToTarget" "SnapToTarget" true)
  (add `/Game/Scripting/Blueprints/Character/BP_FirstPersonCharacter.OnUseItem` (`self.FirstPersonCharacterReference`) (`|CreateDelegate` :!event `OnFireProjectile`))
  ;[1 0.7219 0] Bind for stopping the fire
  (add `/Game/Scripting/Blueprints/Character/BP_FirstPersonCharacter.OnReleasePrimary` (`self.FirstPersonCharacterReference`) (`|CreateDelegate` :!event `CE_Stop Fire`))
  (add `/Game/Scripting/Blueprints/Character/BP_FirstPersonCharacter.OnReload` (`self.FirstPersonCharacterReference`) (`|CreateDelegate` :!event `OnReload`))
  (set `self.MaxOverheat` (`self.Ammo`))
  (set `self.CurrentAmmo` 0.0))

(event `self.SphereCollision.OnComponentBeginOverlap`
  (params (OverlappedComponent :type "PrimitiveComponent Object Reference") (OtherActor :type "Actor Object Reference") (OtherComp :type "PrimitiveComponent Object Reference") (OtherBodyIndex :type Integer) (bFromSweep :type Boolean) (SweepResult :type "HitResult Structure (by ref)"))
  (goto _label))

(event `StartParticle`
  (bind _returnvalue (`NiagaraFunctionLibrary.SpawnSystemAttached` "/Game/FX/Flamethrower/Flamethrower.Flamethrower" (`self.SkeletalMesh`) "Muzzle" (50.0 13.0 -3.0) (struct) "KeepRelativeOffset" true))
  (set `self.Particles` _returnvalue)
  (bind _returnvalue_2 (`GameplayStatics.CreateSound2D` "/Game/Audio/SoundEffects/Weapon/FlameMid_Cue.FlameMid_Cue" 1.0 1.0 0.0 null))
  (bind _output_get (set `self.FlameAudio` _returnvalue_2))
  (`AudioComponent.Play` _output_get 0.0)
  (`PrimitiveComponent.SetMaterial` (`/Game/Scripting/Blueprints/Character/BP_FirstPersonCharacter.FirstPersonMesh` (`self.PlayerRef`)) 0 "/Game/Meshes/Weapons/Materials/Flamethrower/Glow/M_Flamethrower_Glow.M_Flamethrower_Glow"))

(event `CE_Stop Fire`
  (bind _camshake (`self.CamShake`))
  ;[1 0.7219 0] Stop firing projectiles
  (`KismetSystemLibrary.K2_ClearAndInvalidateTimerHandle` (`self.FiringTimer`))
  (`self.Stop Particle`)
  ;[1 0.7892 0] Camera Shake
  (`/Engine/EditorBlueprintResources/StandardMacros.IsValid` _camshake
    (:`Is Valid`
      (`PlayerCameraManager.StopCameraShake` (`GameplayStatics.GetPlayerCameraManager` 0) _camshake true))))

(event `self.OnFireProjectile`
  ;[1 0.7219 0] Start Firing projectile
  (if (`self.CanFire123`)
    (bind _returnvalue (`KismetSystemLibrary.K2_SetTimerDelegate` (delegate `CE_FireProj`) 0.05 true))
    (set `self.FiringTimer` _returnvalue)
    (`self.StartParticle`)
    ;[1 0.7892 0] Camera Shake
    (bind _returnvalue_2 (`MatineeCameraShake.StartMatineeCameraShake` (`GameplayStatics.GetPlayerCameraManager` 0) "/Game/Scripting/Blueprints/Weapons/CameraShakeAssets/BP_FlamethrowerCameraShake.BP_FlamethrowerCameraShake_C"))
    (set `self.CamShake` _returnvalue_2)))

(event `Stop Particle`
  (bind _flameaudio (`self.FlameAudio`))
  (bind _particles (`self.Particles`))
  (`/Engine/EditorBlueprintResources/StandardMacros.IsValid` _particles
    (:`Is Valid`
      (`ActorComponent.K2_DestroyComponent` _particles)
      (`/Engine/EditorBlueprintResources/StandardMacros.IsValid` _flameaudio
        (:`Is Valid`
          (`AudioComponent.Stop` _flameaudio)
          (`GameplayStatics.PlaySound2D` "/Game/Audio/SoundEffects/Weapon/FlameEnd_Cue.FlameEnd_Cue" 1.0 1.0 0.0 null null)
          (`PrimitiveComponent.SetMaterial` (`/Game/Scripting/Blueprints/Character/BP_FirstPersonCharacter.FirstPersonMesh` (`self.PlayerRef`)) 0 "/Game/Meshes/Weapons/Materials/Flamethrower/M_Flamethrower.M_Flamethrower"))))))

(event `CE_FireProj`
  (bind _returnvalue (`PlayerCameraManager.GetCameraRotation` (`GameplayStatics.GetPlayerCameraManager` 0)))
  ;[1 0.7219 0] Individual projectile fire
  (`|SpawnActorFromClass` "/Game/Scripting/Blueprints/Weapons/Projectiles/BP_FlameProjectile.BP_FlameProjectile_C" (`KismetMathLibrary.MakeTransform` (+ (`SceneComponent.GetSocketLocation` (`self.SkeletalMesh`) "Ammo") (`KismetMathLibrary.GreaterGreater_VectorRotator` (`self.ProjectileOffset`) _returnvalue)) (`KismetMathLibrary.Conv_VectorToRotator` (`KismetMathLibrary.RandomUnitVectorInEllipticalConeInDegrees` (`KismetMathLibrary.Conv_RotatorToVector` _returnvalue) 2.5 2.5))) "Undefined" "OverrideRootScale" null (`self.BaseDamage`) null)
  (`self.CE_AddOverheat`))

(event `CE_AddOverheat`
  ;[1 0.7219 0] Overheat Flamethrower Logic
  (`KismetSystemLibrary.K2_ClearAndInvalidateTimerHandle` (`self.CoolingTimer`))
  (bind _result (`/Engine/EditorBlueprintResources/StandardMacros.IncrementFloat` (`self.CurrentOverheat`))
    (:`  `
      (set `self.CurrentAmmo` (`self.CurrentOverheat`))
      (`self.AmmoChange`)
      (if (< _result (`self.MaxOverheat`))
        (bind _returnvalue (`KismetSystemLibrary.K2_SetTimerDelegate` (delegate `CE_Cooldown`) (`self.CooldownTime`) :!label _label_2))
        (set `self.TimeUntilCool` _returnvalue)
        (else
          (set `self.CanFire123` false :!label _label_3)
          (`|PlayMontage` (`/Game/Scripting/Blueprints/Character/BP_FirstPersonCharacter.FirstPersonMesh` (`self.FirstPersonCharacterReference`)) "/Game/Animation/Flamethrower/AM_Flamethrower_Overheat.AM_Flamethrower_Overheat"
            (:`then`
              (set `self.Reloading` true)
              (`self.CE_Stop Fire`)
              (goto _label_2))
            (:`OnCompleted`
              ;[1 0.7219 0] Cooldown Flamethrower
              (set `self.CanFire123` true)
              (`KismetSystemLibrary.K2_ClearAndInvalidateTimerHandle` (`self.CoolingTimer`) :!label _label_4)
              (set `self.Reloading` false))))))))

(event `self.OnReload`
  ;[1 0.7219 0] Overheat Flamethrower Logic
  (if (!= (`self.CurrentOverheat`) 0.0)
    (if (not (`self.Reloading`))
      (goto _label_3))))

(event `CE_Cooldown`
  ;[1 0.7219 0] Cooldown Flamethrower
  (bind _returnvalue (`KismetSystemLibrary.K2_SetTimerDelegate` (delegate `CE_IncrementCooldown`) 0.02 true))
  (set `self.CoolingTimer` _returnvalue))

(event `CE_IncrementCooldown`
  (bind _currentoverheat (`self.CurrentOverheat`))
  ;[1 0.7219 0] Cooldown Flamethrower
  (bind _result (`/Engine/EditorBlueprintResources/StandardMacros.DecrementFloat` _currentoverheat)
    (:`  `
      (set `self.CurrentAmmo` _currentoverheat)
      (`self.AmmoChange`)
      (if (== _result 0.0)
        (goto _label_4)))))

(fn `UserConstructionScript`
  (`parent.UserConstructionScript`))