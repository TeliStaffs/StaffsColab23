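; Parent weapon Blueprint that initializes shared stats and player movement settings for melee and gun weapons.
; On BeginPlay it pushes dash values to BP_FirstPersonCharacter, applies the weapon slowdown through its movement component, and calls empty melee and gun setup events.
; It then maps its class to a row name, loads damage, reload, ammo and firing delay from DT_WeaponStats, and signals the ammo change.
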(event `self.ReceiveBeginPlay`
  (bind _returnvalue (`GameplayStatics.GetActorOfClass` "/Game/Scripting/Blueprints/Character/BP_FirstPersonCharacter.BP_FirstPersonCharacter_C"))
  (`/Game/Scripting/Blueprints/Character/BP_FirstPersonCharacter.SetDashVariables` _returnvalue (`self.DashSpeed`) (`self.DashDistance`))
  ;[1 0.7219 0] Sorry for jacking your bp mike! Do whatever with this aslong as its still called
  (`self.CE_SetWeaponMoveSpeed`)
  (`self.BeginPlayMelee`)
  (`self.BeginPlayGuns`)
  ;[1 0.7219 0] Sets up base values from DT_WeaponStats Data table
  (`self.CE_NameChange`)
  (bind _returnvalue_2 (`|GetDataTableRow` "/Game/Scripting/Blueprints/Weapons/DT_WeaponStats.DT_WeaponStats" (`self.Name`))
    (:`then`
      (bind (_damage _reloadtimer _ammo _firingdelay) (break `/Game/Scripting/Blueprints/Weapons/F_WeaponStats` _returnvalue_2))
      (set `self.BaseDamage` _damage)
      (set `self.ReloadTimer` _reloadtimer)
      (set `self.Ammo` _ammo)
      (set `self.FiringDelay` _firingdelay)
      (set `self.CurrentAmmo` (`self.Ammo`))
      (`self.AmmoChange`))
    (:`RowNotFound`
      (`KismetSystemLibrary.PrintString` "WEAPON BASE: Error Data table row not found" true true (struct :`R` 1.0 :`G` 0.113573 :`A` 1.0)))))

(event `BeginPlayMelee`)

(event `BeginPlayGuns`)

(event `CE_SetWeaponMoveSpeed`
  ;[1 0.7219 0] Edits the characters movement speed based on weapon
  (`/Game/Scripting/Blueprints/Character/AC_Movement.CE_ModifySpeed` (`/Game/Scripting/Blueprints/Character/BP_FirstPersonCharacter.AC_Movement` (stale `self.ReceiveBeginPlay` _returnvalue)) (`self.WeaponSlowdown%`) 0.0 "NewEnumerator1"))

(event `CE_NameChange`
  ;[1 0.7219 0] Changes name based on class
  (set `self.Name` (`BlueprintMapLibrary.Map_Find` (`self.Class->WeaponMap`) (`GameplayStatics.GetObjectClass` self))))

(fn `UserConstructionScript`)