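; Parent Blueprint for melee weapons: swings a knife attack and damages what its collision box overlaps, excluding the player character.
; BeginPlayMelee binds to the player's use-item and dash dispatchers, then calls BeginPlayChild, an empty hook like Dashed.
; SwingWeapon, gated by CanHit until montage blend-out, plays sound and animation while enabling collision.
; The first valid overlap applies knife damage, disables collision and broadcasts WeaponCollided.
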(event `self.BeginPlayMelee`
  (bind _playerref (`self.PlayerRef`))
  ;[0.5 0.7 1] Set Up references and event dispatchers, bind control effects for child weapons after parent weapon effects have taken place
  (bind _returnvalue (`GameplayStatics.GetActorOfClass` "/Game/Scripting/Blueprints/Character/BP_FirstPersonCharacter.BP_FirstPersonCharacter_C"))
  (bind _output_get (set `self.PlayerRef` _returnvalue))
  (add `/Game/Scripting/Blueprints/Character/BP_FirstPersonCharacter.OnUseItem` _playerref (`|CreateDelegate` :!event `SwingWeapon`))
  (add `/Game/Scripting/Blueprints/Character/BP_FirstPersonCharacter.OnUseItem` _output_get (`|CreateDelegate` :!event `SwingWeapon`))
  (add `/Game/Scripting/Blueprints/Character/BP_FirstPersonCharacter.OnDash` _playerref (delegate `Dashed`))
  (`PrimitiveComponent.SetCollisionEnabled` (`self.CollisionBox`) "NoCollision")
  (`self.BeginPlayChild`))

(event `Dashed`
  ;[0.5 0.7 1] Set Up references and event dispatchers, bind control effects for child weapons after parent weapon effects have taken place
)

(event `BeginPlayChild`
  ;[0.5 0.7 1] Set Up references and event dispatchers, bind control effects for child weapons after parent weapon effects have taken place
)

(event `SwingWeapon`
  ;[0.5 0.7 1] Swing the weapon based on a set rotation offset (This will be replaced with animations), damage can only be done while swinging
  (if (`self.CanHit`)
    (set `self.CanHit` false)
    (`PrimitiveComponent.SetCollisionEnabled` (`self.CollisionBox`) "QueryAndPhysics")
    (`GameplayStatics.PlaySound2D` "/Game/Audio/SoundEffects/Whoosh/KnifeCue.KnifeCue" 1.0 1.0 0.0 null null)
    (`|PlayMontage` (`/Game/Scripting/Blueprints/Character/BP_FirstPersonCharacter.FirstPersonMesh` (`self.PlayerRef`)) "/Game/Animation/KnifeV2/Knife_Attack_Montage.Knife_Attack_Montage"
      (:`OnCompleted`
        (`PrimitiveComponent.SetCollisionEnabled` (`self.CollisionBox`) "NoCollision"))
      (:`OnBlendOut`
        (set `self.CanHit` true)))))

(event `self.CollisionBox.OnComponentBeginOverlap`
  (params (OverlappedComponent :type "PrimitiveComponent Object Reference") (OtherActor :type "Actor Object Reference") (OtherComp :type "PrimitiveComponent Object Reference") (OtherBodyIndex :type Integer) (bFromSweep :type Boolean) (SweepResult :type "HitResult Structure (by ref)"))
  ;[0.5 0.7 1] Upon Overlap do Damage while swinging
  (bind _asbp_first_person_character (cast `/Game/Scripting/Blueprints/Character/BP_FirstPersonCharacter` OtherActor)
    (:`then`
      (if (not (== _asbp_first_person_character OtherActor))
        (`GameplayStatics.ApplyDamage` OtherActor (`self.Damage`) null (`GameplayStatics.GetPlayerCharacter` 0) "/Game/Scripting/Blueprints/DamageTypes/DamageType_Knife.DamageType_Knife_C" :!label _label)
        (`PrimitiveComponent.SetCollisionEnabled` (`self.CollisionBox`) "NoCollision")
        (`self.WeaponCollided`)))
    (:`CastFailed`
      (goto _label))))

(fn `UserConstructionScript`)