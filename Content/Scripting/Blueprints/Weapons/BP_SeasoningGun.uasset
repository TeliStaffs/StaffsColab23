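; Seasoning shotgun weapon that fires salt on primary and pepper on secondary, each shot type with its own damage type and Niagara effect.
; Both modes share one ammo pool but have separate cooldown timers; reload plays synced montages and timed sounds, then refills.
; Each shot multi-traces random rays within a cone from the camera, applying distance-scaled damage and knockback to Characters, with slight lift to overcome floor friction.
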(event `self.BeginPlayGuns`
  ;[0.5 0.7 1] Set Current Ammo at start and upon reload
  (set `self.CurrentAmmo` (`self.Ammo`)))

(event `self.OnReload`
  ;[0.5 0.7 1] Set Current Ammo at start and upon reload
  ;;[1 0.7219 0] New Ammo system
  (if (not (`self.Reloading`))
    (set `self.Reloading` true)
    (`|PlayMontage` (`/Game/Scripting/Blueprints/Character/BP_FirstPersonCharacter.FirstPersonMesh` (`self.FirstPersonCharacterReference`)) "/Game/Animation/Shotgun/Mtg_ShotgunReload.Mtg_ShotgunReload"
      (:`then`
        (`|PlayMontage` (`self.Shotgun`) "/Game/Animation/Shotgun/Mtg_Shotgun_Weapon_Reload.Mtg_Shotgun_Weapon_Reload"
          (:`then`
            (`KismetSystemLibrary.K2_SetTimerDelegate` (delegate `CE_openclack`) 0.3))
          (:`OnCompleted`
            (`self.Reload`)))))))

(event `Reload`
  ;[0.5 0.7 1] Set Current Ammo at start and upon reload
  ;;[1 0.7219 0] New Ammo system
  (set `self.CurrentAmmo` (`self.Ammo`))
  (set `self.Reloading` false)
  (`self.AmmoChange`))

(event `CE_openclack`
  (`GameplayStatics.PlaySound2D` "/Game/Audio/SoundEffects/Weapon/WoodenShotgunOpen.WoodenShotgunOpen" 1.0 1.0 0.0 null null)
  (`KismetSystemLibrary.Delay` 1.2)
  (`GameplayStatics.PlaySound2D` "/Game/Audio/SoundEffects/Weapon/Shaker1_Cue.Shaker1_Cue" 1.0 1.0 0.0 null null)
  (`KismetSystemLibrary.Delay` 0.1)
  (`GameplayStatics.PlaySound2D` "/Game/Audio/SoundEffects/Weapon/Shaker1_Cue.Shaker1_Cue" 1.0 1.0 0.0 null null)
  (`KismetSystemLibrary.Delay` 0.1)
  (`GameplayStatics.PlaySound2D` "/Game/Audio/SoundEffects/Weapon/Shaker1_Cue.Shaker1_Cue" 1.0 1.0 0.0 null null)
  (`KismetSystemLibrary.Delay` 0.1)
  (`GameplayStatics.PlaySound2D` "/Game/Audio/SoundEffects/Weapon/Shaker1_Cue.Shaker1_Cue" 1.0 1.0 0.0 null null)
  (`KismetSystemLibrary.Delay` 0.55)
  (`GameplayStatics.PlaySound2D` "/Game/Audio/SoundEffects/Weapon/WoodenShotgunOpen.WoodenShotgunOpen" 1.0 1.0 0.0 null null))

(event `self.OnFireProjectile`
  ;[1 0.7219 0] Fire delay and reload
  (if (`self.CanFire123`)
    (if (`self.Canfiresalt`)
      (set `self.Canfiresalt` false)
      (`KismetSystemLibrary.K2_SetTimerDelegate` (delegate `ResetFireS`) (`self.FiringDelay`))
      ;[0.5 0.7 1] Set Salt or Pepper based on input, if out of ammo, do not fire
      (if (not (`self.Reloading`))
        (set `self.System Template` "/Game/FX/Seasons_Greetings/FX_Salt.FX_Salt")
        (set `self.DamageType` "/Game/Scripting/Blueprints/DamageTypes/DamageType_Salt.DamageType_Salt_C")
        (if (not (<= (`self.CurrentAmmo`) 0.0))
          (set `self.CurrentAmmo` (- (`self.CurrentAmmo`) 1.0))
          (`self.Fire` :!label _label)
          (`self.AmmoChange`)
          (`GameplayStatics.PlaySound2D` "/Game/Audio/SoundEffects/Weapon/SeasoningShotgunSound_Temp__Cue.SeasoningShotgunSound_Temp__Cue" 1.0 1.0 0.0 null null))))))

(event `ResetFireS`
  ;[1 0.7219 0] Fire delay and reload
  (set `self.Canfiresalt` true))

(event `self.OnSecondaryAction`
  ;[1 0.7219 0] Fire delay and reload
  (if (`self.CanFire123`)
    (if (`self.Canfirepepper`)
      (set `self.Canfirepepper` false)
      (`KismetSystemLibrary.K2_SetTimerDelegate` (delegate `CE_ResetFireP`) (`self.FiringDelay`))
      ;[0.5 0.7 1] Set Salt or Pepper based on input, if out of ammo, do not fire
      (if (not (`self.Reloading`))
        (set `self.System Template` "/Game/FX/Seasons_Greetings/FX_Pepper.FX_Pepper")
        (set `self.DamageType` "/Game/Scripting/Blueprints/DamageTypes/DamageType_Pepper.DamageType_Pepper_C")
        (if (not (<= (`self.CurrentAmmo`) 0.0))
          (set `self.CurrentAmmo` (- (`self.CurrentAmmo`) 1.0))
          (goto _label))))))

(event `CE_ResetFireP`
  ;[1 0.7219 0] Fire delay and reload
  (set `self.Canfirepepper` true))

(event `Fire`
  (bind _firespread (`self.FireSpread`))
  (bind _basedamage (`self.BaseDamage`))
  (bind _returnvalue (`PlayerCameraManager.GetCameraRotation` (`GameplayStatics.GetPlayerCameraManager` 0)))
  (bind _returnvalue_2 (`PlayerCameraManager.GetCameraLocation` (`GameplayStatics.GetPlayerCameraManager` 0)))
  (bind (_returnvalue_x _returnvalue_y) (`KismetMathLibrary.BreakVector` (* (`SceneComponent.K2_GetComponentRotation` (`PlayerCameraManager.TransformComponent` (`GameplayStatics.GetPlayerCameraManager` 0))) (* (`self.KnockDistance`) (`self.KnockBackForce`)))))
  ;[1 0.7219 0] Animation and ScreenShake
  (`|PlayMontage` (`/Game/Scripting/Blueprints/Character/BP_FirstPersonCharacter.FirstPersonMesh` (`self.FirstPersonCharacterReference`)) "/Game/Animation/Shotgun/Shotgun_Fire_Montage.Shotgun_Fire_Montage" 1.5
    (:`then`
      (`MatineeCameraShake.StartMatineeCameraShake` (`GameplayStatics.GetPlayerCameraManager` 0) "/Game/Scripting/Blueprints/Weapons/CameraShakeAssets/BP_ShotgunCameraShake.BP_ShotgunCameraShake_C")
      ;[0.5 0.7 1] Fire spread of shots, damage type switches based on primary or secondary shot
      (`NiagaraFunctionLibrary.SpawnSystemAtLocation` (`self.System Template`) (`SceneComponent.K2_GetComponentLocation` (`self.Arrow`)) (`KismetMathLibrary.MakeRotator` (.roll (`PlayerCameraManager.GetCameraRotation` (`GameplayStatics.GetPlayerCameraManager` 0))) (+ (.pitch (`PlayerCameraManager.GetCameraRotation` (`GameplayStatics.GetPlayerCameraManager` 0))) 0.0) (.yaw (`PlayerCameraManager.GetCameraRotation` (`GameplayStatics.GetPlayerCameraManager` 0)))))
      (for _ (range (`self.ShotsPerFire`))
        (bind _outhits (`KismetSystemLibrary.LineTraceMulti` _returnvalue_2 (+ (* (`KismetMathLibrary.RandomUnitVectorInEllipticalConeInDegrees` (`KismetMathLibrary.Conv_RotatorToVector` _returnvalue) _firespread _firespread) 10000.0) (+ _returnvalue_2 (* _returnvalue 1000.0))) "TraceTypeQuery2" false (`|MakeArray` (`self.FirstPersonCharacterReference`) :!type "Actor Object Reference")))
        (for _array_element _outhits
          (bind (_bblockinghit _binitialoverlap _time _distance _location _impactpoint _normal _impactnormal _physmat _hitactor) (`GameplayStatics.BreakHitResult` _array_element))
          (bind _returnvalue_3 (- 1.0 (/ _distance (`self.Max Effective Range`))))
          (set `self.KnockDistance` _returnvalue_3)
          ;[0.5 0.7 1] Launch enemies backwards when they get hit. Add slight Z impulse so the floor friction doesn't prevent them from moving
          (bind _ascharacter (cast `Character` _hitactor))
          (bind _returnvalue_4 (`self.GetComponentByClass` _ascharacter "/Script/Engine.CharacterMovementComponent"))
          (`/Engine/EditorBlueprintResources/StandardMacros.IsValid` _returnvalue_4
            (:`Is Valid`
              (`CharacterMovementComponent.AddImpulse` _returnvalue_4 (`KismetMathLibrary.MakeVector` _returnvalue_x _returnvalue_y 20.0) true)
              ;[0.5 0.7 1] MIKE !! (Apply damage to each actor hit)
              (`GameplayStatics.ApplyDamage` _hitactor (`KismetMathLibrary.FClamp` (* _basedamage _returnvalue_3) 0.0 _basedamage) null (`self.FirstPersonCharacterReference`) (`self.DamageType`)))))))))

(fn `UserConstructionScript`
  (`parent.UserConstructionScript`))