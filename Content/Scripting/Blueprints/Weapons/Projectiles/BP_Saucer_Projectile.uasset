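; BP_Saucer_Projectile is a weapon projectile that captures enemies as ingredients for the current recipe.
; On BeginPlay it caches the recipe keys from the BP_Till in the level.
; On overlap it ignores the player, and if an enemy's IngredientType matches a key, it calls Capture on the enemy's ACHealth and destroys both actors.
; Non-matching enemies are left untouched, as the "Wrong Ingredient!" floating text spawn is unconnected.
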(event `self.CollisionComponent.OnComponentBeginOverlap`
  (params (OverlappedComponent :type "PrimitiveComponent Object Reference") (OtherActor :type "Actor Object Reference") (OtherComp :type "PrimitiveComponent Object Reference") (OtherBodyIndex :type Integer) (bFromSweep :type Boolean) (SweepResult :type "HitResult Structure (by ref)"))
  ;[1 0.7219 0] Get stats from enemy and store them, then destroy the enemy (This will be used later to fill ingredients)
  (cast `/Game/Scripting/Blueprints/Character/BP_FirstPersonCharacter` OtherActor
    (:`CastFailed`
      (bind _asbase_enemy_character (cast `/Game/Scripting/Blueprints/Enemys/BaseEnemy_Character` OtherActor))
      ;[0.5 0.7 1] Check to make sure the ingredient captured was one in the recipe
      (for _array_element (stale `self.ReceiveBeginPlay` _keys)
        (if (`|EnumEquality` _array_element (`/Game/Scripting/Blueprints/Enemys/BaseEnemy_Character.IngredientType` _asbase_enemy_character))
          (set `self.InRecipe` true)
          (break)
          (else
            (set `self.InRecipe` false))))
      (if (`self.InRecipe`)
        ;[0.5 0.7 1] Store Enemy Information (Ingredient Type, Perfection Level)
        (`/Game/Scripting/Blueprints/Enemys/Health/AC_Health.Capture` (`/Game/Scripting/Blueprints/Enemys/BaseEnemy_Character.AC_Health` _asbase_enemy_character))
        ;[0.5 0.7 1] Destroy Actors
        (`self.K2_DestroyActor` _asbase_enemy_character)
        (`self.K2_DestroyActor`)))))

(event `self.ReceiveBeginPlay`
  ;[0.5 0.7 1] Get the Stored Recipe when created
  (bind _returnvalue (`GameplayStatics.GetActorOfClass` "/Game/Scripting/Blueprints/Scoring/BP_Till.BP_Till_C"))
  (bind _output_get (set `self.Recipe` (`/Game/Scripting/Blueprints/Scoring/BP_Till.Recipe` _returnvalue)))
  (bind _keys (`BlueprintMapLibrary.Map_Keys` _output_get)))

(fn `UserConstructionScript`)