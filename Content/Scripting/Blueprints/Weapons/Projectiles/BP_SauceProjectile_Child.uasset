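; Child sauce projectile that bursts on impact, with SpawnCluster overridden empty to stop infinite cluster spawning.
; It launches along its local velocity and enables overlap events after a short delay.
; Its first overlap runs a sphere trace, slowing and damaging AC_Movement owners, using HitArray to skip repeats.
; When the trace hits anything, it spawns a BP_SauceSludge and ketchup Niagara effect just below itself.
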(event `self.ReceiveBeginPlay`
  (`ProjectileMovementComponent.SetVelocityInLocalSpace` (`self.ProjectileMovement`) (`self.velocity`))
  (`KismetSystemLibrary.Delay` 0.5)
  (set `PrimitiveComponent.bGenerateOverlapEvents` true (`self.CollisionComponent`))
  (bind _asbp_first_person_character (cast `/Game/Scripting/Blueprints/Character/BP_FirstPersonCharacter` (`GameplayStatics.GetPlayerCharacter` 0)))
  (set `self.As BP First Person Character` _asbp_first_person_character))

(event `self.SpawnCluster`
  ;[1 0.7219 0] StopsInfiniteLoop DONOTREMOVE
)

(event `self.CollisionComponent.OnComponentBeginOverlap`
  (params (OverlappedComponent :type "PrimitiveComponent Object Reference") (OtherActor :type "Actor Object Reference") (OtherComp :type "PrimitiveComponent Object Reference") (OtherBodyIndex :type Integer) (bFromSweep :type Boolean) (SweepResult :type "HitResult Structure (by ref)"))
  (bind _hitarray (`self.HitArray`))
  (bind _returnvalue (`SceneComponent.K2_GetComponentLocation` (`self.CollisionComponent`)))
  ;[1 0.7219 0] MultiSphereTrace
  (`/Engine/EditorBlueprintResources/StandardMacros.DoOnce` false
    (:`Completed`
      (bind (_outhits _returnvalue_2) (`KismetSystemLibrary.SphereTraceMultiForObjects` :`Start` _returnvalue :`End` _returnvalue :`Radius` (`self.ClusterRadius`) :`ObjectTypes` (`|MakeArray` "ObjectTypeQuery1" "ObjectTypeQuery2" "ObjectTypeQuery3" :!type "EObjectTypeQuery Enum") :`DrawTime` 2.0))
      (if _returnvalue_2
        (for _array_element _outhits
          (bind _returnvalue_3 (`self.GetComponentByClass` (`.HitActor` (`GameplayStatics.BreakHitResult` _array_element)) "/Game/Scripting/Blueprints/Character/AC_Movement.AC_Movement_C"))
          ;[1 0.7219 0] ChecksIfCharacterOrEnvironment
          (`/Engine/EditorBlueprintResources/StandardMacros.IsValid` _returnvalue_3
            (:`Is Valid`
              ;[1 0.7219 0] Slowdowns And Damage
              (if (`KismetArrayLibrary.Array_IsValidIndex` _hitarray)
                (if (not (`KismetArrayLibrary.Array_Contains` _hitarray _returnvalue_3))
                  (`/Game/Scripting/Blueprints/Character/AC_Movement.CE_ModifySpeed` _returnvalue_3 0.5 1.2 "NewEnumerator2")
                  (`GameplayStatics.ApplyDamage` (`.HitActor` (`GameplayStatics.BreakHitResult` _array_element)) (`self.SauceDamage`) null (`self.As BP First Person Character`) "/Game/Scripting/Blueprints/DamageTypes/DamageType_Sauce.DamageType_Sauce_C")
                  (`KismetArrayLibrary.Array_Add` (`self.HitArray`) _returnvalue_3))))))
        (`self.CE_SpawnGoop`)))))

(event `CE_SpawnGoop`
  (bind _returnvalue (- (`self.K2_GetActorLocation`) (0.0 0.0 7.0)))
  (`|SpawnActorFromClass` "/Game/Scripting/Blueprints/Weapons/Projectiles/BP_SauceSludge.BP_SauceSludge_C" (`KismetMathLibrary.MakeTransform` _returnvalue) "Undefined" "OverrideRootScale" null (`self.SauceDamage`) 30.0 null)
  (`NiagaraFunctionLibrary.SpawnSystemAtLocation` "/Game/FX/Sauce_Dispatcher/Ketchup.Ketchup" _returnvalue))

(fn `UserConstructionScript`
  (`parent.UserConstructionScript`))