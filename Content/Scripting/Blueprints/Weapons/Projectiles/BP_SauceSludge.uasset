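; Short-lived sauce puddle that slows and repeatedly damages actors with AC_Movement, crediting the player character, then destroys itself.
; Overlap adds the actor to EnemyArray, applies the slow and an immediate hit, and starts a looping damage timer.
; On exit, it checks every other sludge's array before lifting the slow, so overlapping puddles keep it.
; On spawn, a downward trace tilts it to the surface normal; edge-distance traces are unused.
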(event `self.Collision.OnComponentBeginOverlap`
  (params (OverlappedComponent :type "PrimitiveComponent Object Reference") (OtherActor :type "Actor Object Reference") (OtherComp :type "PrimitiveComponent Object Reference") (OtherBodyIndex :type Integer) (bFromSweep :type Boolean) (SweepResult :type "HitResult Structure (by ref)"))
  (bind _returnvalue (`self.GetComponentByClass` OtherActor "/Game/Scripting/Blueprints/Character/AC_Movement.AC_Movement_C"))
  ;[1 0.7219 0] Begin the overlap
  (`KismetSystemLibrary.PrintString` "Overlap")
  (`/Engine/EditorBlueprintResources/StandardMacros.IsValid` _returnvalue
    (:`Is Valid`
      (`KismetArrayLibrary.Array_AddUnique` (`self.EnemyArray`) OtherActor)
      (`/Game/Scripting/Blueprints/Character/AC_Movement.CE_ModifySpeed` _returnvalue 0.4 0.0 "NewEnumerator2")
      ;[1 0.7219 0] DamageStuf
      (`GameplayStatics.ApplyDamage` OtherActor (`self.SauceDamage`) null (`self.As BP First Person Character`) "/Game/Scripting/Blueprints/DamageTypes/DamageType_Sauce.DamageType_Sauce_C")
      (bind _returnvalue_2 (`KismetSystemLibrary.K2_SetTimerDelegate` (`|CreateDelegate` :!event `DamageTick`) (`self.DamageFrequency`) true))
      (set `self.Damage Tick` _returnvalue_2))))

(event `DamageTick`
  ;[1 0.7219 0] DamageStuf
  (for _array_element (`self.EnemyArray`)
    (`GameplayStatics.ApplyDamage` _array_element (`self.SauceDamage`) null (`self.As BP First Person Character`) "/Game/Scripting/Blueprints/DamageTypes/DamageType_Sauce.DamageType_Sauce_C")))

(event `self.Collision.OnComponentEndOverlap`
  (params (OverlappedComponent :type "PrimitiveComponent Object Reference") (OtherActor :type "Actor Object Reference") (OtherComp :type "PrimitiveComponent Object Reference") (OtherBodyIndex :type Integer))
  (bind _returnvalue (`self.GetComponentByClass` OtherActor "/Game/Scripting/Blueprints/Character/AC_Movement.AC_Movement_C"))
  ;[1 0.7219 0] End Overlap and check if its still overlapped with other sludges
  (`KismetArrayLibrary.Array_RemoveItem` (`self.EnemyArray`) OtherActor)
  (set `self.IsStillSludged` false)
  (`self.CE_IsStillSludgeCheck`)
  (if (not (`self.IsStillSludged`))
    (`/Engine/EditorBlueprintResources/StandardMacros.IsValid` _returnvalue
      (:`Is Valid`
        (`/Game/Scripting/Blueprints/Character/AC_Movement.CE_RemoveSlowType` _returnvalue "NewEnumerator2")
        (if (`KismetArrayLibrary.Array_IsEmpty` (`self.EnemyArray`))
          (`KismetSystemLibrary.K2_ClearAndInvalidateTimerHandle` (`self.Damage Tick`)))))))

(event `CE_IsStillSludgeCheck`
  ;[1 0.7219 0] End Overlap and check if its still overlapped with other sludges
  (bind _outactors (`GameplayStatics.GetAllActorsOfClass` "BP_SauceSludge_C"))
  (for _array_element _outactors
    (if (`KismetArrayLibrary.Array_Contains` (`/Game/Scripting/Blueprints/Weapons/Projectiles/BP_SauceSludge.EnemyArray` _array_element) (stale `self.Collision.OnComponentEndOverlap` OtherActor))
      (set `self.IsStillSludged` true))))

(event `self.ReceiveBeginPlay`
  ;[1 0.7219 0] Initialise and destroy
  (`KismetSystemLibrary.K2_SetTimerDelegate` (delegate `CE_Destroy`) 5.0)
  (`self.CE_SludgeRotate`)
  (bind _asbp_first_person_character (cast `/Game/Scripting/Blueprints/Character/BP_FirstPersonCharacter` (`GameplayStatics.GetPlayerCharacter` 0)))
  (set `self.As BP First Person Character` _asbp_first_person_character))

(event `CE_Destroy`
  ;[1 0.7219 0] Initialise and destroy
  (`self.K2_DestroyActor`))

(event `CE_SludgeRotate`
  (bind _collision (`self.Collision`))
  (bind _collision_2 (`self.Collision`))
  (bind _returnvalue (`SceneComponent.K2_GetComponentLocation` _collision))
  ;[1 0.7219 0] Rotate the sludge
  (bind (_outhit _returnvalue_2) (`KismetSystemLibrary.LineTraceSingleForObjects` _returnvalue (- _returnvalue (* (`SceneComponent.GetUpVector` _collision) 50.0)) (`|MakeArray` "ObjectTypeQuery2" "ObjectTypeQuery1" :!type "EObjectTypeQuery Enum")))
  (if _returnvalue_2
    (`KismetSystemLibrary.PrintString` "Did Hit")
    (bind (_bblockinghit _binitialoverlap _time _distance _location _impactpoint _normal _impactnormal) (`GameplayStatics.BreakHitResult` _outhit))
    (`SceneComponent.K2_SetWorldRotation` _collision_2 (`KismetMathLibrary.MakeRotator` (.roll (`KismetMathLibrary.MakeRotFromXZ` (`SceneComponent.GetForwardVector` _collision_2) _impactnormal)) (.pitch (`KismetMathLibrary.MakeRotFromYZ` (`SceneComponent.GetRightVector` _collision_2) _impactnormal)) (.yaw (`SceneComponent.K2_GetComponentRotation` _collision_2))) false false)))

(event `CE_CheckDistance`
  (if (< (`self.TempDistance`) (`self.CurrentFurthest`))
    (set `self.CurrentFurthest` (`self.TempDistance`))))

(fn `UserConstructionScript`)