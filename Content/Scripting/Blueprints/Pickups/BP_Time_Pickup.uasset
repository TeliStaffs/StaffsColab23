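; BP_Time_Pickup is an extra-time pickup that adds time to the game mode's timer.
; It is a child Blueprint that implements ChildPickupTrigger and keeps the parent's construction script.
; On trigger, it casts to BP_FirstPersonGameMode, increases Time by TimeIncreaseNumber, waits for PickupDuration, then destroys itself.
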(event `self.ChildPickupTrigger`
  ;[1 0 1] Extra Time Pickup
  (bind _asbp_first_person_game_mode (cast `/Game/Scripting/Blueprints/GameMode/BP_FirstPersonGameMode` (`GameplayStatics.GetGameMode`)))
  (set `/Game/Scripting/Blueprints/GameMode/BP_FirstPersonGameMode.Time` (+ (`/Game/Scripting/Blueprints/GameMode/BP_FirstPersonGameMode.Time` _asbp_first_person_game_mode) (`self.timeIncreaseNumber`)) _asbp_first_person_game_mode)
  (`KismetSystemLibrary.Delay` (`self.pickupDuration`))
  (`self.K2_DestroyActor`))

(fn `UserConstructionScript`
  (`parent.UserConstructionScript`))