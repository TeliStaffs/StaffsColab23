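; BP_Jump_Pickup is a child pickup Blueprint that grants the player a temporary double jump with altered jump strength.
; When ChildPickupTrigger fires, it sets the player's jump count to two, caches the movement component's JumpZVelocity and multiplies it by JumpStrength.
; After a PickupDuration delay, it resets the jump count to one and restores the cached velocity.
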(event `self.ChildPickupTrigger`
  (bind _playerrefrence (`self.playerRefrence`))
  ;[1 0 1] Double Jump Pickup
  (set `/Game/Scripting/Blueprints/Character/BP_FirstPersonCharacter.numberOfJumps` 2 _playerrefrence)
  (bind _output_get (set `self.playerCMRefrence` (`Character.CharacterMovement` _playerrefrence)))
  (bind _jumpzvelocity (`CharacterMovementComponent.JumpZVelocity` _output_get))
  (set `self.tmpJumpZVelocity` _jumpzvelocity)
  (set `CharacterMovementComponent.JumpZVelocity` (* _jumpzvelocity (`self.jumpStrength`)) (`self.playerCMRefrence`))
  (`KismetSystemLibrary.Delay` (`self.pickupDuration`))
  (set `/Game/Scripting/Blueprints/Character/BP_FirstPersonCharacter.numberOfJumps` 1 (`self.playerRefrence`))
  (set `CharacterMovementComponent.JumpZVelocity` (`self.tmpJumpZVelocity`) (`self.playerCMRefrence`)))

(fn `UserConstructionScript`
  (`parent.UserConstructionScript`))