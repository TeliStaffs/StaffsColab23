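; Speed pickup Blueprint, a child pickup that temporarily boosts the player's movement speed.
; When the parent's trigger event fires, it calls the modify-speed event on the player's movement component, passing the speed increase negated as a slowdown for the pickup duration.
; The actor waits out that duration before destroying itself.
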(event `self.ChildPickupTrigger`
  ;[1 0 1] Speed Pickup
  (`/Game/Scripting/Blueprints/Character/AC_Movement.CE_ModifySpeed` (`/Game/Scripting/Blueprints/Character/BP_FirstPersonCharacter.AC_Movement` (`self.playerRefrence`)) (* (`self.speedIncrease`) -1.0) (`self.pickupDuration`) "NewEnumerator0")
  (`KismetSystemLibrary.Delay` (`self.pickupDuration`))
  (`self.K2_DestroyActor`))

(fn `UserConstructionScript`
  (`parent.UserConstructionScript`))