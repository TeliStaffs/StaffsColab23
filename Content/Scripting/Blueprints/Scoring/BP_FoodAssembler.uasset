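; Food assembler station that turns cooked ingredients into the final cooking score and ends the game.
; On BeginPlay it binds to BP_Till to store the recipe's required amounts.
; Its box overlap records each ingredient's type and quality, then destroys it.
; A one-time Interact culls surplus best-first via reverse-index removal, so the worst count, then totals quality points and passes the score to BP_FirstPersonGameMode before calling End.
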(event `self.ReceiveBeginPlay`
  ;[0.5 0.7 1] When the till is activated, store the chosen recipe here
  (bind _returnvalue (`GameplayStatics.GetActorOfClass` "/Game/Scripting/Blueprints/Scoring/BP_Till.BP_Till_C"))
  (add `/Game/Scripting/Blueprints/Scoring/BP_Till.SetRecipe` _returnvalue (delegate `SetRecipe`)))

(event `SetRecipe`
  ;[0.5 0.7 1] When the till is activated, store the chosen recipe here
  (bind _output_get (set `self.Recipe` (`/Game/Scripting/Blueprints/Scoring/BP_Till.Recipe` (stale `self.ReceiveBeginPlay` _returnvalue))))
  (bind _keys (`BlueprintMapLibrary.Map_Keys` _output_get))
  (bind _values (`BlueprintMapLibrary.Map_Values` _output_get))
  ;[0.5 0.7 1] Store The Amounts of each ingredient needed
  (for (_array_element _array_index) _keys
    (switch `/Game/Scripting/Blueprints/Enemys/Enums/E_IngredientType` _array_element
      (:`NewEnumerator0`
        (bind _output (`|GetArrayItem` _values _array_index))
        (set `self.BaconAmount` _output))
      (:`NewEnumerator1`
        (set `self.FishNTarTarAmount` _output))
      (:`NewEnumerator2`
        (set `self.SteakAmount` _output))
      (:`NewEnumerator3`
        (set `self.ChipsAmount` _output))
      (:`NewEnumerator4`
        (set `self.ChoppedVegAmount` _output))
      (:`NewEnumerator5`
        (set `self.SeasonedEggAmount` _output))
      (:`NewEnumerator6`
        (set `self.SmallMeatAmount` _output))
      (:`NewEnumerator8`
        (set `self.RoasterAmount` _output))
      (:`NewEnumerator9`
        (set `self.BatteredFishAmount` _output))
      (:`NewEnumerator10`
        (set `self.RoasternGravyAmount` _output))
      (:`NewEnumerator12`
        (set `self.SlicedFishAmount` _output)))))

(event `/Game/Scripting/Blueprints/Scoring/BPI_Interact.Interact`
  (bind _allingredientlevels (`self.AllIngredientLevels`))
  ;[0.5 0.7 1] Loop through the stored ingredients, find the worst quality of each ingredient in the number that is needed, remove the rest
  (if (`self.IngredientStored`)
    (`/Engine/EditorBlueprintResources/StandardMacros.DoOnce` false
      (:`Completed`
        (bind _newperfectionlevelarray (`self.CullIngredient` (`self.BaconPerfectionLevel`) (`self.BaconAmount`)))
        (bind _output_get (set `self.BaconPerfectionLevel` _newperfectionlevelarray))
        (bind _newperfectionlevelarray_2 (`self.CullIngredient` (`self.FishnTarTarPerfectionLevel`) (`self.FishNTarTarAmount`)))
        (bind _output_get_2 (set `self.FishnTarTarPerfectionLevel` _newperfectionlevelarray_2))
        (bind _newperfectionlevelarray_3 (`self.CullIngredient` (`self.SteakPerfectionLevel`) (`self.SteakAmount`)))
        (bind _output_get_3 (set `self.SteakPerfectionLevel` _newperfectionlevelarray_3))
        (bind _newperfectionlevelarray_4 (`self.CullIngredient` (`self.ChipsPerfectionLevel`) (`self.ChipsAmount`)))
        (bind _output_get_4 (set `self.ChipsPerfectionLevel` _newperfectionlevelarray_4))
        (bind _newperfectionlevelarray_5 (`self.CullIngredient` (`self.ChoppedVegPerfectionLevel`) (`self.ChoppedVegAmount`)))
        (bind _output_get_5 (set `self.ChoppedVegPerfectionLevel` _newperfectionlevelarray_5))
        (bind _newperfectionlevelarray_6 (`self.CullIngredient` (`self.SeasonedEggPerfectionLevel`) (`self.SeasonedEggAmount`)))
        (bind _output_get_6 (set `self.SeasonedEggPerfectionLevel` _newperfectionlevelarray_6))
        (bind _newperfectionlevelarray_7 (`self.CullIngredient` (`self.SmallMeatPerfectionLevel`) (`self.SmallMeatAmount`)))
        (bind _output_get_7 (set `self.SmallMeatPerfectionLevel` _newperfectionlevelarray_7))
        (bind _newperfectionlevelarray_8 (`self.CullIngredient` (`self.RoasterPerfectionLevel`) (`self.RoasterAmount`)))
        (bind _output_get_8 (set `self.RoasterPerfectionLevel` _newperfectionlevelarray_8))
        (bind _newperfectionlevelarray_9 (`self.CullIngredient` (`self.BatteredFishPerfectionLevel`) (`self.BatteredFishAmount`)))
        (bind _output_get_9 (set `self.BatteredFishPerfectionLevel` _newperfectionlevelarray_9))
        (bind _newperfectionlevelarray_10 (`self.CullIngredient` (`self.RoastersNGravyPerfectionLevel`) (`self.RoasternGravyAmount`)))
        (bind _output_get_10 (set `self.RoastersNGravyPerfectionLevel` _newperfectionlevelarray_10))
        (bind _newperfectionlevelarray_11 (`self.CullIngredient` (`self.SlicedFishPerfectionLevel`) (`self.SlicedFishAmount`)))
        (bind _output_get_11 (set `self.SlicedFishPerfectionLevel` _newperfectionlevelarray_11))
        ;[0.5 0.7 1] Combine all of the saved perfection levels into one array so they can be cycled through and score calculated
        (for _array_element _output_get
          (`KismetArrayLibrary.Array_Add` _allingredientlevels _array_element))
        (for _array_element_2 _output_get_2
          (`KismetArrayLibrary.Array_Add` _allingredientlevels _array_element_2))
        (for _array_element_3 _output_get_3
          (`KismetArrayLibrary.Array_Add` _allingredientlevels _array_element_3))
        (for _array_element_4 _output_get_4
          (`KismetArrayLibrary.Array_Add` _allingredientlevels _array_element_4))
        (for _array_element_5 _output_get_5
          (`KismetArrayLibrary.Array_Add` _allingredientlevels _array_element_5))
        (for _array_element_6 _output_get_6
          (`KismetArrayLibrary.Array_Add` _allingredientlevels _array_element_6))
        (for _array_element_7 _output_get_7
          (`KismetArrayLibrary.Array_Add` _allingredientlevels _array_element_7))
        (for _array_element_8 _output_get_8
          (`KismetArrayLibrary.Array_Add` _allingredientlevels _array_element_8))
        (for _array_element_9 _output_get_9
          (`KismetArrayLibrary.Array_Add` _allingredientlevels _array_element_9))
        (for _array_element_10 _output_get_10
          (`KismetArrayLibrary.Array_Add` _allingredientlevels _array_element_10))
        (for _array_element_11 _output_get_11
          (`KismetArrayLibrary.Array_Add` _allingredientlevels _array_element_11))
        ;[0.5 0.7 1] Calculate the scores of each ingredient left and combine them to get the final cooking score
        (for _array_element_12 (`self.AllIngredientLevels`)
          (if (`|EnumEquality` _array_element_12 "NewEnumerator0")
            (set `self.CookingScore` (+ (`self.CookingScore`) (`self.PerfectIngredientScore`)))
            (elif (`|EnumEquality` _array_element_12 "NewEnumerator1")
              (set `self.CookingScore` (+ (`self.CookingScore`) (`self.GoodIngredientScore`)))
              (elif (`|EnumEquality` _array_element_12 "NewEnumerator2")
                (set `self.CookingScore` (+ (`self.CookingScore`) (`self.OkayIngredientScore`)))
                (elif (`|EnumEquality` _array_element_12 "NewEnumerator3")
                  (set `self.CookingScore` (+ (`self.CookingScore`) (`self.BadIngredientScore`))))))))
        (bind _asbp_first_person_game_mode (cast `/Game/Scripting/Blueprints/GameMode/BP_FirstPersonGameMode` (`GameplayStatics.GetGameMode`)))
        (`/Game/Scripting/Blueprints/GameMode/BP_FirstPersonGameMode.SetCookingScore` _asbp_first_person_game_mode (`self.CookingScore`))
        (`/Game/Scripting/Blueprints/GameMode/BP_FirstPersonGameMode.End` _asbp_first_person_game_mode)))))

(event `self.Box.OnComponentBeginOverlap`
  (params (OverlappedComponent :type "PrimitiveComponent Object Reference") (OtherActor :type "Actor Object Reference") (OtherComp :type "PrimitiveComponent Object Reference") (OtherBodyIndex :type Integer) (bFromSweep :type Boolean) (SweepResult :type "HitResult Structure (by ref)"))
  ;[0.5 0.7 1] Store perfection levels for each type of ingredient as it enters
  (bind _asbp_cooked_enemy_ingredient (cast `/Game/Scripting/Blueprints/Enemys/BP_CookedEnemyIngredient` OtherActor))
  (set `self.IngredientStored` true)
  (switch `/Game/Scripting/Blueprints/Enemys/Enums/E_IngredientType` (`/Game/Scripting/Blueprints/Enemys/BP_CookedEnemyIngredient.IngredientType` _asbp_cooked_enemy_ingredient)
    (:`NewEnumerator11`
      (`KismetSystemLibrary.PrintString` "Assembler: Ingredient Does Not Match Stored Ingredient Type" true true (struct :`R` 0.5 :`G` 0.7 :`B` 1.0 :`A` 1.0)))
    (:`NewEnumerator0`
      (bind _perfectionlevel (`/Game/Scripting/Blueprints/Enemys/BP_CookedEnemyIngredient.PerfectionLevel` _asbp_cooked_enemy_ingredient))
      (`KismetArrayLibrary.Array_Add` (`self.BaconPerfectionLevel`) _perfectionlevel))
    (:`NewEnumerator1`
      (`KismetArrayLibrary.Array_Add` (`self.FishnTarTarPerfectionLevel`) _perfectionlevel))
    (:`NewEnumerator2`
      (`KismetArrayLibrary.Array_Add` (`self.SteakPerfectionLevel`) _perfectionlevel))
    (:`NewEnumerator3`
      (`KismetArrayLibrary.Array_Add` (`self.ChipsPerfectionLevel`) _perfectionlevel))
    (:`NewEnumerator4`
      (`KismetArrayLibrary.Array_Add` (`self.ChoppedVegPerfectionLevel`) _perfectionlevel))
    (:`NewEnumerator5`
      (`KismetArrayLibrary.Array_Add` (`self.SeasonedEggPerfectionLevel`) _perfectionlevel))
    (:`NewEnumerator6`
      (`KismetArrayLibrary.Array_Add` (`self.SmallMeatPerfectionLevel`) _perfectionlevel))
    (:`NewEnumerator8`
      (`KismetArrayLibrary.Array_Add` (`self.RoasterPerfectionLevel`) _perfectionlevel))
    (:`NewEnumerator9`
      (`KismetArrayLibrary.Array_Add` (`self.BatteredFishPerfectionLevel`) _perfectionlevel))
    (:`NewEnumerator10`
      (`KismetArrayLibrary.Array_Add` (`self.RoastersNGravyPerfectionLevel`) _perfectionlevel))
    (:`NewEnumerator12`
      (`KismetArrayLibrary.Array_Add` (`self.SlicedFishPerfectionLevel`) _perfectionlevel)))
  (`self.K2_DestroyActor` OtherActor))

(fn `CullIngredient`
  (params (PerfectionLevelArray :type "Array of /Game/Scripting/Blueprints/Enemys/Health/E_PerfectionLevel Enum") (IngredientAmount :type Integer))
  (returns (NewPerfectionLevelArray :type "Array of /Game/Scripting/Blueprints/Enemys/Health/E_PerfectionLevel Enum"))
  (locals (PerfectionLevels :type "Array of /Game/Scripting/Blueprints/Enemys/Health/E_PerfectionLevel Enum") (IngredientAmounts :type Integer))
  (bind _indexarray (`self.IndexArray`))
  (bind _perfectionlevels (`local.PerfectionLevels`))
  (bind _indexarray_2 (`self.IndexArray`))
  (bind _indexarray_3 (`self.IndexArray`))
  (bind _indexarray_4 (`self.IndexArray`))
  (bind _indexarray_5 (`self.IndexArray`))
  (bind _indexarray_6 (`self.IndexArray`))
  (bind _indexarray_7 (`self.IndexArray`))
  (bind _indexarray_8 (`self.IndexArray`))
  ;[0.5 0.7 1] Check how many of the ingredient type are required. If more than that amount have been stored, store the indexes of the highest quality in an array, and remove them until the correct amount is met. If the quanity of stored ingredients is still too high, move down the next highest quality and do the same
  (set `local.PerfectionLevels` PerfectionLevelArray)
  (set `local.IngredientAmounts` IngredientAmount)
  (for (_array_element _array_index) PerfectionLevelArray
    (if (`|EnumEquality` _array_element "NewEnumerator0")
      (`KismetArrayLibrary.Array_Add` _indexarray_7 _array_index)))
  (`KismetArrayLibrary.Array_Reverse` _indexarray_7)
  (for _array_element_2 _indexarray_8
    (if (> (`KismetArrayLibrary.Array_Length` (`local.PerfectionLevels`)) (`local.IngredientAmounts`))
      (`KismetArrayLibrary.Array_Remove` _perfectionlevels _array_element_2)))
  (`KismetArrayLibrary.Array_Clear` _indexarray_8)
  (for _ _perfectionlevels
    _)
  ;[0.5 0.7 1] Remove Good Quality ingredients until correct amount remain
  (for (_array_element_3 _array_index_2) (`local.PerfectionLevels`)
    (if (`|EnumEquality` _array_element_3 "NewEnumerator1")
      (`KismetArrayLibrary.Array_Add` _indexarray_2 _array_index_2)))
  (`KismetArrayLibrary.Array_Reverse` _indexarray_2)
  (for _array_element_4 _indexarray_3
    (if (> (`KismetArrayLibrary.Array_Length` (`local.PerfectionLevels`)) (`local.IngredientAmounts`))
      (`KismetArrayLibrary.Array_Remove` (`local.PerfectionLevels`) _array_element_4)))
  (`KismetArrayLibrary.Array_Clear` _indexarray_3)
  ;[0.5 0.7 1] Remove Okay Quality ingredients until correct amount remain
  (for (_array_element_5 _array_index_3) (`local.PerfectionLevels`)
    (if (`|EnumEquality` _array_element_5 "NewEnumerator2")
      (`KismetArrayLibrary.Array_Add` _indexarray_4 _array_index_3)))
  (`KismetArrayLibrary.Array_Reverse` _indexarray_4)
  (for _array_element_6 _indexarray_5
    (if (> (`KismetArrayLibrary.Array_Length` (`local.PerfectionLevels`)) (`local.IngredientAmounts`))
      (`KismetArrayLibrary.Array_Remove` (`local.PerfectionLevels`) _array_element_6)))
  (`KismetArrayLibrary.Array_Clear` _indexarray_5)
  ;[0.5 0.7 1] Remove Bad Quality ingredients until correct amount remain
  (for (_array_element_7 _array_index_4) (`local.PerfectionLevels`)
    (if (`|EnumEquality` _array_element_7 "NewEnumerator3")
      (`KismetArrayLibrary.Array_Add` _indexarray _array_index_4)))
  (`KismetArrayLibrary.Array_Reverse` _indexarray)
  (for _array_element_8 _indexarray_6
    (if (> (`KismetArrayLibrary.Array_Length` (`local.PerfectionLevels`)) (`local.IngredientAmounts`))
      (`KismetArrayLibrary.Array_Remove` (`local.PerfectionLevels`) _array_element_8)))
  (`KismetArrayLibrary.Array_Clear` _indexarray_6)
  (return (`local.PerfectionLevels`)))

(fn `UserConstructionScript`)