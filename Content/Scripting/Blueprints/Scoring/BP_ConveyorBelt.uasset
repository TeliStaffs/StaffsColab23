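; Conveyor belt that, once started by its button, pushes characters along it, but only if every ingredient in the recipe has been collected.
; It copies the recipe from BP_Till when notified, and GetIngredient decrements the remaining count of each captured type.
; A button press runs CheckInventory; if nothing remains, a fast looping timer applies forward velocity-change impulses to overlapping CharacterMovementComponents in PushBox.
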(event `self.ReceiveBeginPlay`
  ;[0.5 0.7 1] Set Up wisgets and recipe
  (bind _returnvalue (`GameplayStatics.GetActorOfClass` "/Game/Scripting/Blueprints/Scoring/BP_Till.BP_Till_C"))
  (add `/Game/Scripting/Blueprints/Scoring/BP_Till.SetRecipe` _returnvalue (delegate `Set Up`))
  ;[1 0 0] Must have conveyor button in scene
  (add `/Game/Scripting/Blueprints/Scoring/BP_Button.StartConveyer` (`self.Button`) (delegate `Start`)))

(event `Set Up`
  ;[0.5 0.7 1] Set Up wisgets and recipe
  (set `self.Recipe` (`/Game/Scripting/Blueprints/Scoring/BP_Till.Recipe` (stale `self.ReceiveBeginPlay` _returnvalue))))

(event `Start`
  ;[0.5 0.7 1] Move object across conveyor belt
  (bind _allingredients (`self.CheckInventory`))
  (if _allingredients
    (`KismetSystemLibrary.K2_SetTimerDelegate` (delegate `Push Ingredients`) 0.01 true)))

(event `GetIngredient`
  (params (IngredientType :type "/Game/Scripting/Blueprints/Enemys/Enums/E_IngredientType Enum" :default "NewEnumerator0"))
  (bind _recipe (`self.Recipe`))
  ;[0.5 0.7 1] The same as in the WBP Recipe, tick off ingredients as they are captured, when you have at least the correct amount of each, the conveyor belt can be used, called in game mode
  (bind _keys (`BlueprintMapLibrary.Map_Keys` _recipe))
  (for (_array_element _array_index) _keys
    (if (`|EnumEquality` _array_element IngredientType)
      (bind _values (`BlueprintMapLibrary.Map_Values` (`self.Recipe`)))
      (bind _output (`|GetArrayItem` _values _array_index))
      (if (> _output 0)
        (`BlueprintMapLibrary.Map_Add` _recipe _array_element (- _output 1))))))

(event `Push Ingredients`
  ;[0.5 0.7 1] Move object across conveyor belt
  (for _array_element (`PrimitiveComponent.GetOverlappingActors` (`self.PushBox`) null)
    (bind _returnvalue (`self.GetComponentByClass` _array_element "/Script/Engine.CharacterMovementComponent"))
    ;;[0.9893 1 0] Check is valid
    (`/Engine/EditorBlueprintResources/StandardMacros.IsValid` _returnvalue
      (:`Is Valid`
        (`CharacterMovementComponent.AddImpulse` _returnvalue (* (`KismetMathLibrary.Conv_RotatorToVector` (`SceneComponent.K2_GetComponentRotation` (`self.DefaultSceneRoot`))) (`self.ConveyorBeltForce`)) true)))))

(fn `CheckInventory`
  (returns (AllIngredients :type Boolean))
  (locals (IngredientCheck :type Boolean))
  ;[0.5 0.7 1] Loop through recipe values, if there is at least one of an ingredient remaining, ingredient check is set to false. If no ingredients are needed, set to true.
  (bind _values (`BlueprintMapLibrary.Map_Values` (`self.Recipe`)))
  (for _array_element _values
    (if (!= _array_element 0)
      (set `local.IngredientCheck` false)
      (break)
      (else
        (set `local.IngredientCheck` true))))
  (return (`local.IngredientCheck`)))

(fn `UserConstructionScript`)