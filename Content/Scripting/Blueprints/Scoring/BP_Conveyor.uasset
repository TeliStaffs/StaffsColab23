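; BP_Conveyor is a conveyor belt actor meant to push characters along its forward direction.
; Actor begin overlap sets a non-looping, zero-time timer bound to CE_Move, rather than pushing continuously on Tick.
; CE_Move loops over actors overlapping the static mesh and gives each CharacterMovementComponent a velocity-change impulse along the root's X axis, scaled by ConveyorBeltForce.
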(event `self.ReceiveActorBeginOverlap`
  (params (OtherActor :type "Actor Object Reference"))
  (`KismetSystemLibrary.K2_SetTimerDelegate` (delegate `CE_Move`)))

(event `CE_Move`
  (for _array_element (`PrimitiveComponent.GetOverlappingActors` (`self.StaticMesh`) null)
    (bind _returnvalue (`self.GetComponentByClass` _array_element "/Script/Engine.CharacterMovementComponent"))
    ;[0.9893 1 0] Check is valid
    (`/Engine/EditorBlueprintResources/StandardMacros.IsValid` _returnvalue
      (:`Is Valid`
        (`CharacterMovementComponent.AddImpulse` _returnvalue (* (`KismetMathLibrary.Conv_RotatorToVector` (`SceneComponent.K2_GetComponentRotation` (`self.DefaultSceneRoot`))) (`self.ConveyorBeltForce`)) true)))))

(fn `UserConstructionScript`)