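; Interactable button that calls a conveyor start once pressed and clears valid voice timers on all teleporters in the level.
; It becomes active when the game mode signals that all ingredients are collected, though Interact itself does not check that flag.
; Box overlap by the player toggles custom-depth highlighting and swaps the HUD crosshair between default, "E" and a tinted "Inactive" prompt.
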(event `self.ReceiveBeginPlay`
  (bind _outactors (`GameplayStatics.GetAllActorsOfClass` "/Game/Scripting/Blueprints/Teleportation/BP_Teleporter.BP_Teleporter_C"))
  (set `self.Out Actors` _outactors)
  (bind _asbp_first_person_character (cast `/Game/Scripting/Blueprints/Character/BP_FirstPersonCharacter` (`GameplayStatics.GetPlayerCharacter` 0)))
  (set `self.Player` _asbp_first_person_character)
  (set `self.Crosshair` (`/Game/Scripting/Blueprints/Character/WBP_Crosshair.Crosshair` (`/Game/UI/Widgets/WBP_HUD.WBP_Crosshair` (`/Game/Scripting/Blueprints/Character/BP_FirstPersonCharacter.PlayerHUD` _asbp_first_person_character))))
  (bind _asbp_first_person_game_mode (cast `/Game/Scripting/Blueprints/GameMode/BP_FirstPersonGameMode` (`GameplayStatics.GetGameMode`)))
  (bind _output_get (set `self.GM` _asbp_first_person_game_mode))
  (add `/Game/Scripting/Blueprints/GameMode/BP_FirstPersonGameMode.AllIngredientsCollected` _output_get (delegate `MakeActive`)))

(event `MakeActive`
  (params (Result :type Boolean))
  (set `self.isActive?` true))

(event `/Game/Scripting/Blueprints/Scoring/BPI_Interact.Interact`
  (`self.StartConveyer`)
  (for _array_element (`self.Out Actors`)
    (`/Engine/EditorBlueprintResources/StandardMacros.IsValid` _array_element
      (:`Is Valid`
        (bind _voicetimer (`/Game/Scripting/Blueprints/Teleportation/BP_Teleporter.VoiceTimer` _array_element))
        (if (`KismetSystemLibrary.K2_IsValidTimerHandle` _voicetimer)
          (`KismetSystemLibrary.K2_ClearAndInvalidateTimerHandle` _voicetimer))))))

(event `self.Box.OnComponentBeginOverlap`
  (params (OverlappedComponent :type "PrimitiveComponent Object Reference") (OtherActor :type "Actor Object Reference") (OtherComp :type "PrimitiveComponent Object Reference") (OtherBodyIndex :type Integer) (bFromSweep :type Boolean) (SweepResult :type "HitResult Structure (by ref)"))
  (bind _crosshair (`self.Crosshair`))
  ;[0.1927 0 0] Interaction prompt
  (if (== OtherActor (`self.Player`))
    (`PrimitiveComponent.SetRenderCustomDepth` (`self.StaticMesh`) true)
    (if (`self.isActive?`)
      (`TextBlock.SetText` _crosshair "E")
      (else
        (`TextBlock.SetText` _crosshair "Inactive")
        (`TextBlock.SetColorAndOpacity` _crosshair (`self.InactiveColour`))))))

(event `self.Box.OnComponentEndOverlap`
  (params (OverlappedComponent :type "PrimitiveComponent Object Reference") (OtherActor :type "Actor Object Reference") (OtherComp :type "PrimitiveComponent Object Reference") (OtherBodyIndex :type Integer))
  (bind _crosshair (`self.Crosshair`))
  ;[0.1927 0 0] Interaction prompt
  (if (== (`self.Player`) OtherActor)
    (`TextBlock.SetText` _crosshair "+")
    (`PrimitiveComponent.SetRenderCustomDepth` (`self.StaticMesh`) false)
    (`TextBlock.SetColorAndOpacity` _crosshair (`self.Normal`))))

(fn `UserConstructionScript`)