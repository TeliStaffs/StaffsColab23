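; BP_Till is an interactable till that assigns the player a random recipe once.
; Its box overlap highlights the mesh and text and switches the HUD crosshair to an interact or inactive prompt.
; Interact draws a random DT_Recipes row, passes it to the HUD, and broadcasts SetRecipe for other Blueprints, including teleporter activation.
; It also triggers an alien voice line, then deactivates the till and displays the recipe name in red.
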(event `self.Box.OnComponentBeginOverlap`
  (params (OverlappedComponent :type "PrimitiveComponent Object Reference") (OtherActor :type "Actor Object Reference") (OtherComp :type "PrimitiveComponent Object Reference") (OtherBodyIndex :type Integer) (bFromSweep :type Boolean) (SweepResult :type "HitResult Structure (by ref)"))
  (bind _crosshair (`self.Crosshair`))
  ;[0.1927 0 0] Interaction prompt
  (if (and (== OtherActor (`self.Player`)) (`self.isActive`))
    (`PrimitiveComponent.SetRenderCustomDepth` (`self.StaticMesh`) true)
    (`TextBlock.SetText` _crosshair "E")
    (`TextRenderComponent.SetTextRenderColor` (`self.TextRender`) (`self.Glow`))
    (else
      (`TextBlock.SetText` _crosshair "Inactive")
      (`TextBlock.SetColorAndOpacity` _crosshair (`self.InactiveColour`)))))

(event `self.Box.OnComponentEndOverlap`
  (params (OverlappedComponent :type "PrimitiveComponent Object Reference") (OtherActor :type "Actor Object Reference") (OtherComp :type "PrimitiveComponent Object Reference") (OtherBodyIndex :type Integer))
  (bind _crosshair (`self.Crosshair`))
  ;[0.1927 0 0] Interaction prompt
  (if (== (`self.Player`) OtherActor)
    (`TextBlock.SetText` _crosshair "+")
    (`PrimitiveComponent.SetRenderCustomDepth` (`self.StaticMesh`) false)
    (`TextBlock.SetColorAndOpacity` _crosshair (`self.In Color and Opacity_0`))
    (`TextRenderComponent.SetTextRenderColor` (`self.TextRender`) (`self.Default`))))

(event `self.ReceiveBeginPlay`
  ;[1 0.7892 0] Alien Voice Manager
  (bind _returnvalue (`GameplayStatics.GetActorOfClass` "/Game/Scripting/Blueprints/TutorialLevel/BP_AlienVoiceManager.BP_AlienVoiceManager_C"))
  (`/Engine/EditorBlueprintResources/StandardMacros.IsValid` _returnvalue
    (:`Is Valid`
      (set `self.AVM` _returnvalue)
      ;[0.1927 0 0] CrosshairRef
      (bind _asbp_first_person_character (cast `/Game/Scripting/Blueprints/Character/BP_FirstPersonCharacter` (`GameplayStatics.GetPlayerCharacter` 0)))
      (set `self.Player` _asbp_first_person_character)
      (set `self.Crosshair` (`/Game/Scripting/Blueprints/Character/WBP_Crosshair.Crosshair` (`/Game/UI/Widgets/WBP_HUD.WBP_Crosshair` (`/Game/Scripting/Blueprints/Character/BP_FirstPersonCharacter.PlayerHUD` _asbp_first_person_character)))))))

(event `/Game/Scripting/Blueprints/Scoring/BPI_Interact.Interact`
  (bind _avm (`self.AVM`))
  (bind _textrender (`self.TextRender`))
  (bind _recipename (`self.RecipeName`))
  ;[0.5 0.7 1] Will Set the recipe and send a message to other blueprints, telling them to set the recipe, will also allow teleporters to become functional
  (`/Engine/EditorBlueprintResources/StandardMacros.DoOnce` false
    (:`Completed`
      ;;[1 0.7892 0] Alien VoiceManager
      (`/Engine/EditorBlueprintResources/StandardMacros.IsValid` _avm
        (:`Is Valid`
          (`/Game/UI/Widgets/I_Objective.SetNewText` _avm "Now human, go step on my teleporter or else."))
        (:`Is Not Valid`
          _))
      (bind _asbp_first_person_character (cast `/Game/Scripting/Blueprints/Character/BP_FirstPersonCharacter` (`GameplayStatics.GetPlayerCharacter` 0)))
      (set `self.Player HUD` (`/Game/Scripting/Blueprints/Character/BP_FirstPersonCharacter.PlayerHUD` _asbp_first_person_character))
      (bind _outrownames (`DataTableFunctionLibrary.GetDataTableRowNames` "/Game/Scripting/Blueprints/Recipes/DT_Recipes.DT_Recipes"))
      (bind _output_get (set `self.RecipeName` (`KismetArrayLibrary.Array_Random` _outrownames)))
      (`/Game/UI/Widgets/WBP_Switcher.GetRecipe` (`/Game/UI/Widgets/WBP_HUD.WBP_Switcher` (`self.Player HUD`)) _output_get)
      (bind _returnvalue (`|GetDataTableRow` "/Game/Scripting/Blueprints/Recipes/DT_Recipes.DT_Recipes" _recipename)
        (:`then`
          (set `self.Recipe` (`.Recipe_8_90B99CC045854F32ABB1DC81A9D7A2BF` (break `/Game/Scripting/Blueprints/Recipes/F_Recipe` _returnvalue)))
          (`self.SetRecipe`)
          ;[0.1927 0 0] Inactive recipe counter
          (set `self.isActive` false)
          (`TextRenderComponent.SetTextRenderColor` _textrender (`self.Red`))
          (`TextRenderComponent.K2_SetText` _textrender (`KismetTextLibrary.Conv_NameToText` _recipename)))))))

(fn `UserConstructionScript`)