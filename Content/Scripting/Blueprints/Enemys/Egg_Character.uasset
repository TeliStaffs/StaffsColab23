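; Egg enemy character that periodically hops in place.
; BeginPlay starts a looping timer, with an interval picked once at random between a few seconds and ten, that fires the Hop event.
; Hop replays a timeline that lerps the actor toward a point above its current location without sweep.
; The lerp re-reads location on every update, so the lift is relative rather than measured from a stored start.
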(event `self.ReceiveBeginPlay`
  (`parent.ReceiveBeginPlay`)
  (`KismetSystemLibrary.K2_SetTimerDelegate` (delegate `Hop!`) (`KismetMathLibrary.RandomFloatInRange` 3.0 10.0) true))

(event `self.ReceiveTick`
  (params (DeltaSeconds :type "Float (single-precision)")))

(event `Hop!`
  (bind (_returnvalue_x _returnvalue_y _returnvalue_z) (`KismetMathLibrary.BreakVector` (`self.K2_GetActorLocation`)))
  (bind (_direction _newtrack_0) (`Timeline|Hop` :!via `PlayFromStart`)
    (:`Update`
      (`self.K2_SetActorLocation` (`KismetMathLibrary.VLerp` (`self.K2_GetActorLocation`) (`KismetMathLibrary.MakeVector` _returnvalue_x _returnvalue_y (+ _returnvalue_z 50.0)) _newtrack_0)))))

(fn `UserConstructionScript`
  (`parent.UserConstructionScript`))