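; Meat enemy character that splits into two small meats once it has been chopped enough.
; On any damage it runs the parent handling, then reads the perfection level from its health component.
; When that level's type and grade match the chopping threshold, it disables capsule collision, spawns two SmallMeat_Character actors at its own transform and destroys itself.
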(event `self.ReceiveAnyDamage`
  (params (Damage :type "Float (single-precision)") (DamageType :type "DamageType Object Reference") (InstigatedBy :type "Controller Object Reference") (DamageCauser :type "Actor Object Reference"))
  (bind _ac_health (`self.AC_Health`))
  (bind _capsulecomponent (`self.CapsuleComponent`))
  (bind _returnvalue (`SceneComponent.K2_GetComponentToWorld` _capsulecomponent))
  ;[0.5 0.7 1] When a sufficient chopping level has been reached, will split into two small meats
  (`parent.ReceiveAnyDamage` Damage DamageType InstigatedBy DamageCauser)
  (`/Engine/EditorBlueprintResources/StandardMacros.IsValid` _ac_health
    (:`Is Valid`
      (bind (_perfectionenum _wbpperfectionfloat _type) (`/Game/Scripting/Blueprints/Enemys/Health/AC_Health.GetPerfectionLevel` _ac_health))
      (`/Engine/EditorBlueprintResources/StandardMacros.IsValid` _ac_health
        (:`Is Valid`
          (if (and (`|EnumEquality` _type "NewEnumerator0") (`|EnumEquality` _perfectionenum "NewEnumerator0"))
            (`PrimitiveComponent.SetCollisionEnabled` _capsulecomponent "NoCollision")
            (`|SpawnActorFromClass` "/Game/Scripting/Blueprints/Enemys/SmallMeat_Character.SmallMeat_Character_C" _returnvalue "AdjustIfPossibleButAlwaysSpawn" "OverrideRootScale" null null)
            (`|SpawnActorFromClass` "/Game/Scripting/Blueprints/Enemys/SmallMeat_Character.SmallMeat_Character_C" _returnvalue "AdjustIfPossibleButAlwaysSpawn" "OverrideRootScale" null null)
            (`self.K2_DestroyActor`)))))))

(fn `UserConstructionScript`
  (`parent.UserConstructionScript`))