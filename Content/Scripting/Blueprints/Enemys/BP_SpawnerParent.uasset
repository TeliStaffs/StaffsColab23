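; Parent enemy spawner actor that spawns one type of enemy when the game mode requests it.
; On BeginPlay it binds its Spawn event to the SpawnNewEnemies dispatcher on BP_FirstPersonGameMode.
; When the broadcast class matches its EnemyType, it spawns that class at the center of its Box bounds, ignoring collisions.
; A random navigable-point lookup is present but unused.
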(event `self.ReceiveBeginPlay`
  (bind _asbp_first_person_game_mode (cast `/Game/Scripting/Blueprints/GameMode/BP_FirstPersonGameMode` (`GameplayStatics.GetGameMode`)))
  (bind _output_get (set `self.GM` _asbp_first_person_game_mode))
  (add `/Game/Scripting/Blueprints/GameMode/BP_FirstPersonGameMode.SpawnNewEnemies` _output_get (delegate `Spawn`)))

(event `Spawn`
  (params (Class :type "/Game/Scripting/Blueprints/Enemys/Enums/E_EnemyType Enum" :default "NewEnumerator0"))
  (if (`|EnumEquality` (`self.EnemyType`) Class)
    (`|SpawnActorFromClass` (`self.Class`) (`KismetMathLibrary.MakeTransform` (`KismetSystemLibrary.GetComponentBounds` (`self.Box`))) "AlwaysSpawn" "OverrideRootScale" null null)))

(fn `UserConstructionScript`)