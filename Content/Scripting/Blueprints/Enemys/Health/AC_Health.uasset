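; Enemy health component that turns damage into food preparation, tracking flame, salt and pepper, sauce and knife resistances loaded by enemy type.
; Each hit grades that prep type from Raw to Perfect by remaining-resistance bands, with the best band mid-depletion.
; Preps are matched against data-table recipes to pick the resulting ingredient; depleted resistance or incompatible recipes destroy the enemy.
; Capture sends ingredient, averaged perfection and mesh to the game mode.
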(event `self.ReceiveBeginPlay`
  ;[1 0.7219 0] Set Enemy Reference and find data table for character
  (bind _asbase_enemy_character (cast `/Game/Scripting/Blueprints/Enemys/BaseEnemy_Character` (`self.GetOwner`))
    (:`then`
      (set `self.EnemyReference` _asbase_enemy_character)
      (bind _enemytype (`/Game/Scripting/Blueprints/Enemys/BaseEnemy_Character.EnemyType` _asbase_enemy_character))
      (set `self.Enemy Type` _enemytype)
      (bind _returnvalue (`|GetDataTableRow` "/Game/Scripting/Blueprints/Enemys/Health/DT_EnemyResistance.DT_EnemyResistance" (`BlueprintMapLibrary.Map_Find` (`self.EnumMap`) _enemytype))
        (:`then`
          ;[1 0.7219 0] Set values based on F_DamageResistances
          (bind _output_get (set `self.DamageResistances` _returnvalue))
          (`|ExecutionSequence`
            (:`then_0`
              (bind (_flame _saltpepper _sauce _knife) (break `/Game/Scripting/Blueprints/Enemys/Health/F_DamageResistances` _output_get))
              (set `self.MaxFireRes` _flame)
              (set `self.MaxS&PRes` _saltpepper))
            (:`then_1`
              (set `self.MaxSauceRes` _sauce)
              (set `self.MaxSliceRes` _knife))))
        (:`RowNotFound`
          (`KismetSystemLibrary.PrintString` "ERROR AC_Health: RowNotFound" true true (struct :`R` 1.0 :`G` 0.052273 :`A` 1.0)))))
    (:`CastFailed`
      (`KismetSystemLibrary.PrintString` "ERROR AC_Health: AC_Health should only be implemented in enemies" true true (struct :`R` 1.0 :`G` 0.029832 :`A` 1.0)))))

(fn `Average Perfection Amount`
  (locals (BigPerfectionLevel :type "Float (double-precision)") (`Modify Amount` :type "Float (double-precision)") (NumberOfAdditions :type Integer) (FinalPerfectionLevel :type "Float (double-precision)") (CheckVariable :type "Float (double-precision)") (BarModifyAmount :type "Float (double-precision)"))
  (bind (_damageresistances_flame _damageresistances_saltpepper _damageresistances_sauce _damageresistances_knife) (break `/Game/Scripting/Blueprints/Enemys/Health/F_DamageResistances` (`self.DamageResistances`)))
  ;[1 0.7219 0] Find all of the relevant prep types
  (for _array_element (`self.PrepTypeArray`)
    ;[1 0.7219 0] Find Average perfection
    (switch `/Game/Scripting/Blueprints/Enemys/Enums/E_PrepType` _array_element
      (:`NewEnumerator0`
        (set `local.CheckVariable` (- 1.0 (/ _damageresistances_flame (`self.MaxFireRes`)))))
      (:`NewEnumerator1`
        (set `local.CheckVariable` (- 1.0 (/ _damageresistances_knife (`self.MaxSliceRes`)))))
      (:`NewEnumerator2`
        (set `local.CheckVariable` (- 1.0 (/ _damageresistances_saltpepper (`self.MaxS&PRes`)))))
      (:`NewEnumerator3`
        (set `local.CheckVariable` (- 1.0 (/ _damageresistances_sauce (`self.MaxSauceRes`))))))
    (set `local.BarModifyAmount` (`local.CheckVariable`))
    (switch `/Game/Scripting/Blueprints/Enemys/Health/E_PerfectionLevel` (`BlueprintMapLibrary.Map_Find` (`self.Prep Type and Level`) _array_element)
      (:`NewEnumerator4`
        (set `local.Modify Amount` 0.0))
      (:`NewEnumerator0`
        (set `local.Modify Amount` 1.0))
      (:`NewEnumerator1`
        (set `local.Modify Amount` 0.8))
      (:`NewEnumerator2`
        (set `local.Modify Amount` 0.4))
      (:`NewEnumerator3`
        (set `local.Modify Amount` 0.1)))
    (set `local.BigPerfectionLevel` (+ (`local.BigPerfectionLevel`) (`local.Modify Amount`)))
    (`/Engine/EditorBlueprintResources/StandardMacros.IncrementInt` (`local.NumberOfAdditions`)))
  (set `local.FinalPerfectionLevel` (/ (`local.BigPerfectionLevel`) (`local.NumberOfAdditions`)))
  (set `self.SuperPerfectionLevel` (`local.BarModifyAmount`))
  (if (`KismetMathLibrary.InRange_FloatFloat` (`local.FinalPerfectionLevel`) 0.0 0.3 true false)
    (set `self.PerfectionLevel` "NewEnumerator3")
    (elif (`KismetMathLibrary.InRange_FloatFloat` (`local.FinalPerfectionLevel`) 0.3 0.55 true false)
      (set `self.PerfectionLevel` "NewEnumerator2")
      (elif (`KismetMathLibrary.InRange_FloatFloat` (`local.FinalPerfectionLevel`) 0.55 0.8)
        (set `self.PerfectionLevel` "NewEnumerator1")
        (elif (`KismetMathLibrary.InRange_FloatFloat` (`local.FinalPerfectionLevel`) 0.8 1.0 false)
          (set `self.PerfectionLevel` "NewEnumerator0")
          (else
            (`KismetSystemLibrary.PrintString` "AC_Health Error(AveragePerfectionLevel): No perfection level found" true true (struct :`R` 1.0 :`G` 0.006772 :`A` 1.0))))))))

(fn `Capture`
  ;[1 1 0] Send captured data to First Person Character
  (bind _asbp_first_person_game_mode (cast `/Game/Scripting/Blueprints/GameMode/BP_FirstPersonGameMode` (`GameplayStatics.GetGameMode`)))
  (bind _asbase_enemy_character (cast `/Game/Scripting/Blueprints/Enemys/BaseEnemy_Character` (`self.GetOwner`)))
  (`self.Average Perfection Amount`)
  (`/Game/Scripting/Blueprints/GameMode/BP_FirstPersonGameMode.StoreEnemyStats` _asbp_first_person_game_mode (`self.IngredientType`) (`self.PerfectionLevel`) (`SkinnedMeshComponent.SkeletalMesh` (`Character.Mesh` _asbase_enemy_character))))

(fn `CheckCookedStatus`
  (params (TypeToCheck :type "/Game/Scripting/Blueprints/Enemys/Health/E_DamageType Enum" :default "NewEnumerator3"))
  (locals (VarToCheck :type "Float (double-precision)") (DamageType :type "/Game/Scripting/Blueprints/Enemys/Health/E_DamageType Enum" :default "NewEnumerator3") (DMGResPrep :type "Map of /Game/Scripting/Blueprints/Enemys/Enums/E_PrepType Enum to /Game/Scripting/Blueprints/Enemys/Health/E_PerfectionLevel Enum") (MaxVarToCheck :type "Float (double-precision)") (PrepType :type "/Game/Scripting/Blueprints/Enemys/Enums/E_PrepType Enum"))
  (bind (_damageresistances_flame _damageresistances_saltpepper _damageresistances_sauce _damageresistances_knife) (break `/Game/Scripting/Blueprints/Enemys/Health/F_DamageResistances` (`self.DamageResistances`)))
  (bind (_damageresistances_flame_2 _damageresistances_saltpepper_2 _damageresistances_sauce_2 _damageresistances_knife_2 _damageresistances_preptypeandlevel) (break `/Game/Scripting/Blueprints/Enemys/Health/F_DamageResistances` (`self.DamageResistances`)))
  (bind (_flame _saltpepper _sauce _knife) (break `/Game/Scripting/Blueprints/Enemys/Health/F_DamageResistances` (`self.DamageResistances`)))
  ;[1 0.7219 0] SetVariables to be edited
  (bind _output_get (set `local.DamageType` TypeToCheck))
  (switch `/Game/Scripting/Blueprints/Enemys/Health/E_DamageType` _output_get
    (:`NewEnumerator3`
      (set `local.VarToCheck` _damageresistances_flame)
      (set `local.PrepType` "NewEnumerator0")
      (set `local.MaxVarToCheck` (`self.MaxFireRes`)))
    (:`NewEnumerator2`
      (set `local.VarToCheck` _damageresistances_saltpepper)
      (set `local.PrepType` "NewEnumerator2")
      (set `local.MaxVarToCheck` (`self.MaxS&PRes`)))
    (:`NewEnumerator1`
      (set `local.VarToCheck` _damageresistances_sauce)
      (set `local.PrepType` "NewEnumerator3")
      (set `local.MaxVarToCheck` (`self.MaxSauceRes`)))
    (:`NewEnumerator0`
      (set `local.VarToCheck` _damageresistances_knife)
      (set `local.PrepType` "NewEnumerator1")
      (set `local.MaxVarToCheck` (`self.MaxSliceRes`))))
  ;[1 0.7219 0] MATHS!
  (if (<= (`local.VarToCheck`) 0.0)
    (`self.Death`)
    (else
      (set `local.DMGResPrep` _damageresistances_preptypeandlevel)
      (if (or (and (<= (`local.VarToCheck`) (* (`local.MaxVarToCheck`) 0.7)) (> (`local.VarToCheck`) (* (`local.MaxVarToCheck`) 0.5))) (and (<= (`local.VarToCheck`) (* (`local.MaxVarToCheck`) 0.25)) (> (`local.VarToCheck`) (* (`local.MaxVarToCheck`) 0.12))))
        (`BlueprintMapLibrary.Map_Add` (`local.DMGResPrep`) (`local.PrepType`) "NewEnumerator2")
        (set `self.ParticularPerfection` "NewEnumerator2")
        ;[1 0.7219 0] Set The new states
        (set `self.FLOATTEST` (`local.VarToCheck`) :!label _label)
        (set `self.TEST Damage Type` (`local.DamageType`))
        (`self.Average Perfection Amount`)
        (set `self.DamageResistances` (make `/Game/Scripting/Blueprints/Enemys/Health/F_DamageResistances` _flame _saltpepper _sauce _knife (`local.DMGResPrep`)))
        (`self.DebugDamages`)
        (`self.Compare Enums`)
        (elif (or (and (<= (`local.VarToCheck`) (* (`local.MaxVarToCheck`) 0.5)) (> (`local.VarToCheck`) (* (`local.MaxVarToCheck`) 0.4))) (and (<= (`local.VarToCheck`) (* (`local.MaxVarToCheck`) 0.35)) (> (`local.VarToCheck`) (* (`local.MaxVarToCheck`) 0.25))))
          (`BlueprintMapLibrary.Map_Add` (`local.DMGResPrep`) (`local.PrepType`) "NewEnumerator1")
          (set `self.ParticularPerfection` "NewEnumerator1")
          (goto _label)
          (elif (and (<= (`local.VarToCheck`) (* (`local.MaxVarToCheck`) 0.4)) (> (`local.VarToCheck`) (* (`local.MaxVarToCheck`) 0.35)))
            (`BlueprintMapLibrary.Map_Add` (`local.DMGResPrep`) (`local.PrepType`) "NewEnumerator0")
            (set `self.ParticularPerfection` "NewEnumerator0")
            (goto _label)
            (elif (or (and (<= (`local.VarToCheck`) (* (`self.MaxFireRes`) 0.9)) (> (`local.VarToCheck`) (* (`self.MaxFireRes`) 0.7))) (<= (`local.VarToCheck`) (* (`self.MaxFireRes`) 0.12)))
              (`BlueprintMapLibrary.Map_Add` (`local.DMGResPrep`) (`local.PrepType`) "NewEnumerator3")
              (set `self.ParticularPerfection` "NewEnumerator3")
              (goto _label)
              (elif (> (`local.VarToCheck`) (* (`self.MaxFireRes`) 0.9))
                (`BlueprintMapLibrary.Map_Add` (`local.DMGResPrep`) (`local.PrepType`) "NewEnumerator4")
                (goto _label)
                (else
                  (`KismetSystemLibrary.PrintString` "AC_HEALTH ERROR: Cannot detect "))))))))))

(fn `Compare Enums`
  (locals (`Preparation level and Type` :type "Map of /Game/Scripting/Blueprints/Enemys/Enums/E_PrepType Enum to /Game/Scripting/Blueprints/Enemys/Health/E_PerfectionLevel Enum") (CookedCheck :type Boolean :default true) (TempResultIngredient :type "/Game/Scripting/Blueprints/Enemys/Enums/E_IngredientType Enum" :default "NewEnumerator11") (NameVsType :type "Map of /Game/Scripting/Blueprints/Enemys/Enums/E_EnemyType Enum to /Game/Scripting/Blueprints/Enemys/Health/F_TESTING2 Structure") (`Temp Recipe` :type "Array of /Game/Scripting/Blueprints/Enemys/Enums/E_PrepType Enum") (PossibleRecipies :type "Array of /Game/Scripting/Blueprints/Enemys/Enums/E_IngredientType Enum") (Array1 :type "Array of /Game/Scripting/Blueprints/Enemys/Enums/E_PrepType Enum") (BiggerArray :type "Array of /Game/Scripting/Blueprints/Enemys/Enums/E_PrepType Enum") (SmallerArray :type "Array of /Game/Scripting/Blueprints/Enemys/Enums/E_PrepType Enum") (`Recipes Compatible` :type Boolean) (ResultIngredient :type "/Game/Scripting/Blueprints/Enemys/Enums/E_IngredientType Enum" :default "NewEnumerator11") (TestyMcTester :type "Array of Boolean"))
  (bind _array1 (`local.Array1`))
  (bind _temp_recipe (`local.Temp Recipe`))
  (bind (_flame _saltpepper _sauce _knife _preptypeandlevel) (break `/Game/Scripting/Blueprints/Enemys/Health/F_DamageResistances` (`self.DamageResistances`)))
  (set `self.Prep Type and Level` _preptypeandlevel)
  (set `local.Preparation level and Type` _preptypeandlevel)
  (for _array_element (`.PossibleIngredients_8_9A1B75B44386DC8E61B62D925BC60781` (break `/Game/Scripting/Blueprints/Enemys/Health/F_TESTING2` (`BlueprintMapLibrary.Map_Find` (`local.NameVsType`) (`self.Enemy Type`))))
    ;[1 0.7219 0] Loops to check each ingredient type possible for a enemy
    (bind _returnvalue (`|GetDataTableRow` "/Game/Scripting/Blueprints/Enemys/Health/DT_PossibleIngredients.DT_PossibleIngredients" _array_element)
      (:`then`
        (bind (_recipe _resultingredient) (break `/Game/Scripting/Blueprints/Enemys/Health/F_Test` _returnvalue))
        ;[1 0.7219 0] Loops, Checks the base ingredient to see if all the necesarry steps to become an new ingredient have been achieved
        (set `local.TempResultIngredient` _resultingredient)
        (bind _output_get (set `local.Temp Recipe` _recipe))
        (for _array_element_2 _output_get
          (bind (_value _returnvalue_2) (`BlueprintMapLibrary.Map_Find` (`local.Preparation level and Type`) _array_element_2))
          (if (and (`|EnumInequality` _value "NewEnumerator4") _returnvalue_2)
            (set `local.CookedCheck` false)
            (else
              (set `local.CookedCheck` true)
              (break))))
        (if (`local.CookedCheck`)
          _
          (elif (`KismetArrayLibrary.Array_IsNotEmpty` (`local.Array1`))
            ;[1 0.7219 0] Checks to see if the ingredient is still able to become other ingredients/Is a valid ingredient
            (if (not (`KismetArrayLibrary.Array_Identical` _array1 _temp_recipe))
              (if (< (`KismetArrayLibrary.Array_Length` _array1) (`KismetArrayLibrary.Array_Length` _temp_recipe))
                (set `local.SmallerArray` (`local.Array1`))
                (set `local.BiggerArray` (`local.Temp Recipe`))
                (else
                  (set `local.BiggerArray` (`local.Array1`))
                  (set `local.SmallerArray` (`local.Temp Recipe`))))
              (set `local.Recipes Compatible` true)
              (for _array_element_3 (`local.SmallerArray`)
                (if (not (`KismetArrayLibrary.Array_Contains` (`local.BiggerArray`) _array_element_3))
                  (set `local.Recipes Compatible` false)
                  (break)))
              (if (`local.Recipes Compatible`)
                (set `local.Array1` (`local.BiggerArray`))
                (set `local.ResultIngredient` (`local.TempResultIngredient`))
                (if (< (`KismetArrayLibrary.Array_Length` (`local.Array1`)) (`BlueprintMapLibrary.Map_Length` (`local.Preparation level and Type`))) :!label _label
                  _)
                (else
                  (`self.Death`))))
            (else
              (set `local.Array1` _output_get)
              (set `local.ResultIngredient` (`local.TempResultIngredient`))
              (goto _label)))))
      (:`RowNotFound`
        (`KismetSystemLibrary.PrintString` (`KismetStringLibrary.Concat_StrStr` "CE_Health ERROR: Row not found. (CompareEnumsFunction)" (`KismetStringLibrary.Conv_NameToString` _array_element)) true true (struct :`R` 1.0 :`G` 0.051414 :`A` 1.0) 20.0))))
  (set `self.IngredientType` (`local.ResultIngredient`))
  (set `self.PrepTypeArray` (`local.Array1`)))

(fn `Death`
  (bind _returnvalue (`self.GetOwner`))
  (`NiagaraFunctionLibrary.SpawnSystemAtLocation` "/Game/FX/DeathEffect.DeathEffect" (`Actor.K2_GetActorLocation` (`self.GetOwner`)))
  (bind _returnvalue_2 (`GameplayStatics.GetActorOfClass` "/Game/Scripting/Blueprints/Character/BP_FirstPersonCharacter.BP_FirstPersonCharacter_C"))
  (`/Game/UI/Widgets/I_Objective.SetNewText` _returnvalue_2 "Use the Cloche gun (2) to capture enemies!")
  (`/Engine/EditorBlueprintResources/StandardMacros.IsValid` _returnvalue
    (:`Is Valid`
      (`Actor.K2_DestroyActor` _returnvalue))))

(fn `DebugDamages`)

(fn `GetPerfectionLevel`
  (returns (PerfectionEnum :type "/Game/Scripting/Blueprints/Enemys/Health/E_PerfectionLevel Enum") (WBPPerfectionFloat :type "Float (double-precision)") (Type :type "/Game/Scripting/Blueprints/Enemys/Health/E_DamageType Enum") (`Ingredient Type` :type "/Game/Scripting/Blueprints/Enemys/Enums/E_IngredientType Enum") (EnemyType :type "/Game/Scripting/Blueprints/Enemys/Enums/E_EnemyType Enum"))
  (bind _ingredienttype (`self.IngredientType`))
  (bind _perfectionlevel (`self.PerfectionLevel`))
  (`self.Average Perfection Amount`)
  (if (`|EnumInequality` _ingredienttype "NewEnumerator11")
    (return _perfectionlevel (`self.SuperPerfectionLevel`) (`self.TEST Damage Type`) _ingredienttype "NewEnumerator0")
    (else
      (return _perfectionlevel (`self.SuperPerfectionLevel`) (`self.TEST Damage Type`) "NewEnumerator11" (`self.Enemy Type`)))))

(fn `ModifyResistance`
  (params (DamageType :type "DamageType Class Reference") (ModificationAmount :type "Float (double-precision)"))
  (locals (`Current Health` :type "Float (double-precision)" :default 1.0) (`Temp Health` :type "Float (double-precision)") (`Current Change` :type "Float (double-precision)") (DamageTypes :type "/Game/Scripting/Blueprints/Enemys/Health/E_DamageType Enum" :default "NewEnumerator0"))
  (bind (_damageresistances_flame _damageresistances_saltpepper _damageresistances_sauce _damageresistances_knife) (break `/Game/Scripting/Blueprints/Enemys/Health/F_DamageResistances` (`self.DamageResistances`)))
  (bind (_damageresistances_flame_2 _damageresistances_saltpepper_2 _damageresistances_sauce_2 _damageresistances_knife_2 _damageresistances_preptypeandlevel) (break `/Game/Scripting/Blueprints/Enemys/Health/F_DamageResistances` (`self.DamageResistances`)))
  (bind (_damageresistances_flame_3 _damageresistances_saltpepper_3 _damageresistances_sauce_3 _damageresistances_knife_3 _damageresistances_preptypeandlevel_2) (break `/Game/Scripting/Blueprints/Enemys/Health/F_DamageResistances` (`self.DamageResistances`)))
  (bind (_damageresistances_flame_4 _damageresistances_saltpepper_4 _damageresistances_sauce_4 _damageresistances_knife_4 _damageresistances_preptypeandlevel_3) (break `/Game/Scripting/Blueprints/Enemys/Health/F_DamageResistances` (`self.DamageResistances`)))
  (bind (_damageresistances_flame_5 _damageresistances_saltpepper_5 _damageresistances_sauce_5 _damageresistances_knife_5 _damageresistances_preptypeandlevel_4) (break `/Game/Scripting/Blueprints/Enemys/Health/F_DamageResistances` (`self.DamageResistances`)))
  ;[1 0.7219 0] Uses Map to set Damage type enum
  (set `local.Current Change` ModificationAmount)
  (bind _output_get (set `local.DamageTypes` (`BlueprintMapLibrary.Map_Find` (`self.DamageTypeMap`) DamageType)))
  ;[1 0.7219 0] Chooses which 'health' will be damaged
  (switch `/Game/Scripting/Blueprints/Enemys/Health/E_DamageType` _output_get
    (:`NewEnumerator3`
      (set `local.Current Health` _damageresistances_flame))
    (:`NewEnumerator2`
      (set `local.Current Health` _damageresistances_saltpepper))
    (:`NewEnumerator1`
      (set `local.Current Health` _damageresistances_sauce))
    (:`NewEnumerator0`
      (set `local.Current Health` _damageresistances_knife)))
  (set `local.Current Health` (- (`local.Current Health`) (`local.Current Change`)))
  ;[1 0.7219 0] Changes F_DamageResistances
  (switch `/Game/Scripting/Blueprints/Enemys/Health/E_DamageType` (`local.DamageTypes`)
    (:`NewEnumerator3`
      (set `self.DamageResistances` (make `/Game/Scripting/Blueprints/Enemys/Health/F_DamageResistances` (`local.Current Health`) _damageresistances_saltpepper_4 _damageresistances_sauce_4 _damageresistances_knife_4 _damageresistances_preptypeandlevel_3)))
    (:`NewEnumerator2`
      (set `self.DamageResistances` (make `/Game/Scripting/Blueprints/Enemys/Health/F_DamageResistances` _damageresistances_flame_5 (`local.Current Health`) _damageresistances_sauce_5 _damageresistances_knife_5 _damageresistances_preptypeandlevel_4)))
    (:`NewEnumerator1`
      (set `self.DamageResistances` (make `/Game/Scripting/Blueprints/Enemys/Health/F_DamageResistances` _damageresistances_flame_2 _damageresistances_saltpepper_2 (`local.Current Health`) _damageresistances_knife_2 _damageresistances_preptypeandlevel)))
    (:`NewEnumerator0`
      (set `self.DamageResistances` (make `/Game/Scripting/Blueprints/Enemys/Health/F_DamageResistances` _damageresistances_flame_3 _damageresistances_saltpepper_3 _damageresistances_sauce_3 (`local.Current Health`) _damageresistances_preptypeandlevel_2))))
  ;[1 0.7219 0] Calls the Check Cook status function
  (`self.CheckCookedStatus` (`local.DamageTypes`)))