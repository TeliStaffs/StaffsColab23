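; AI controller for enemies that runs the BT_Core behavior tree and drives it through a state enum.
; StateChange copies the state to the blackboard's States key, with extra calls for Wander and Flee.
; Perceived damage switches to Flee, while sight updates reset to Wander unless the AI is fleeing and the sensed actor is the player.
; The hearing branch is empty.
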(event `self.ReceiveBeginPlay`
  (`self.RunBehaviorTree` "/Game/Scripting/Blueprints/Enemys/AI/BT_Core.BT_Core")
  (`self.StateChange`)
  (bind _asbp_first_person_character (cast `/Game/Scripting/Blueprints/Character/BP_FirstPersonCharacter` (`GameplayStatics.GetPlayerCharacter` 0)))
  (set `self.player ref` _asbp_first_person_character))

(event `StateChange`
  (bind _blackboardcomp (`self.BlackboardComp`))
  (bind _state (`self.State`))
  ;[0.2708 0 0.002417] on state change
  (switch `/Game/Scripting/Blueprints/Enemys/Enums/E_EnemyStates` (`self.State`)
    (:`NewEnumerator0`
      ;[0.2708 0 0.002417] Update AI BB
      (`BlackboardComponent.SetValueAsEnum` _blackboardcomp "States" _state)
      (`self.WanderState`))
    (:`NewEnumerator1`
      (`BlackboardComponent.SetValueAsEnum` _blackboardcomp "States" _state)
      (`self.FleeState`))
    (:`NewEnumerator2`
      (`BlackboardComponent.SetValueAsEnum` _blackboardcomp "States" _state))
    (:`NewEnumerator3`
      (`BlackboardComponent.SetValueAsEnum` _blackboardcomp "States" _state))
    (:`NewEnumerator4`
      (`BlackboardComponent.SetValueAsEnum` _blackboardcomp "States" _state))
    (:`NewEnumerator5`
      (`BlackboardComponent.SetValueAsEnum` _blackboardcomp "States" _state))))

(event `self.AIPerception.OnTargetPerceptionUpdated`
  (params (Actor :type "Actor Object Reference") (Stimulus :type "AIStimulus Structure"))
  (bind _returnvalue (`AIPerceptionSystem.GetSenseClassForStimulus` Stimulus))
  ;[0.1927 0 0] Damage
  (if (== _returnvalue "/Script/AIModule.AISense_Damage")
    (set `self.State` "NewEnumerator1")
    (`self.StateChange`)
    (else
      ;[0.1927 0 0] Sight
      (if (== _returnvalue "/Script/AIModule.AISense_Sight")
        (if (`KismetMathLibrary.BooleanNAND` (`|EnumEquality` (`self.State`) "NewEnumerator1") (== Actor (`self.player ref`)))
          (set `self.State` "NewEnumerator0")
          (`self.StateChange`))
        (else
          ;[0.1927 0 0] Hearing
          (if (== _returnvalue "/Script/AIModule.AISense_Hearing")
            _))))))

(fn `UserConstructionScript`)