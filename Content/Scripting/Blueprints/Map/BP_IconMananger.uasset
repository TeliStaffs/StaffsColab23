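; Map icon actor that shows a chosen Paper2D sprite and is meant to toggle it with the player's map.
; On BeginPlay it sets the sprite, caches the first-person character and binds to its OnMapToggle event.
; The UpdateIconVisibility1 event matches sprite visibility to the character's MapToggled flag.
; The UpdateIconVisibility function called at the end of BeginPlay is empty, so that call sets no initial visibility.
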(event `self.ReceiveBeginPlay`
  ;[1 0 1] Toggle map icons on and off
  (`PaperSpriteComponent.SetSprite` (`self.PaperSprite`) (`self.chosenIcon`))
  (bind _asbp_first_person_character (cast `/Game/Scripting/Blueprints/Character/BP_FirstPersonCharacter` (`GameplayStatics.GetPlayerCharacter` 0)))
  (bind _output_get (set `self.As BP First Person Character` _asbp_first_person_character))
  (add `/Game/Scripting/Blueprints/Character/BP_FirstPersonCharacter.OnMapToggle` _output_get (`|CreateDelegate` :!event `UpdateIconVisibility1`))
  (`self.UpdateIconVisibility`))

(event `UpdateIconVisibility1`
  (bind _papersprite (`self.PaperSprite`))
  ;[1 0 1] Toggle map icons on and off
  (if (`/Game/Scripting/Blueprints/Character/BP_FirstPersonCharacter.mapToggled?` (`self.As BP First Person Character`))
    (`SceneComponent.SetVisibility` _papersprite true false)
    (else
      (`SceneComponent.SetVisibility` _papersprite false false))))

(fn `UpdateIconVisibility`)

(fn `UserConstructionScript`)