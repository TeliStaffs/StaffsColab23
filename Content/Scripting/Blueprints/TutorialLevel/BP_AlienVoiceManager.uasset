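; BP_AlienVoiceManager drives the aliens' talking text widget on the player HUD in the tutorial level.
; On BeginPlay it caches that widget and binds to the game mode's all-ingredients-collected event and the conveyor belt's speak event.
; Each trigger passes a line to SetNewText, which cancels the hide timer, calls CallNewVoiceLine and shows the widget.
; FinishedText starts a timer that hides the widget after a delay.
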(event `self.ReceiveBeginPlay`
  (`KismetSystemLibrary.Delay` 0.1)
  (bind _asbp_first_person_character (cast `/Game/Scripting/Blueprints/Character/BP_FirstPersonCharacter` (`GameplayStatics.GetPlayerCharacter` 0))
    (:`then`
      (bind _wbp_alienstalking (`/Game/UI/Widgets/WBP_HUD.WBP_AliensTalking` (`/Game/Scripting/Blueprints/Character/BP_FirstPersonCharacter.PlayerHUD` _asbp_first_person_character)))
      (set `self.WBP Aliens Talking` _wbp_alienstalking)
      (`Widget.SetIsEnabled` _wbp_alienstalking true)
      (bind _asbp_first_person_game_mode (cast `/Game/Scripting/Blueprints/GameMode/BP_FirstPersonGameMode` (`GameplayStatics.GetGameMode`)))
      (add `/Game/Scripting/Blueprints/GameMode/BP_FirstPersonGameMode.AllIngredientsCollected` _asbp_first_person_game_mode (delegate `CE_ingredientCOllected`))
      (bind _returnvalue (`GameplayStatics.GetActorOfClass` "/Game/Scripting/Blueprints/ConveyorBelt/BP_ConveyorBelt.BP_ConveyorBelt_C"))
      (`/Engine/EditorBlueprintResources/StandardMacros.IsValid` _returnvalue
        (:`Is Valid`
          (add `/Game/Scripting/Blueprints/ConveyorBelt/BP_ConveyorBelt.SpeakToMe` _returnvalue (delegate `CE_Conveyor Speak`)))))
    (:`CastFailed`
      (`KismetSystemLibrary.PrintString` "Cast Failed"))))

(event `CE_Conveyor Speak`
  (`/Game/UI/Widgets/I_Objective.SetNewText` (`self.ConveyorLine`)))

(event `CE_ingredientCOllected`
  (params (Result :type Boolean))
  (`/Game/UI/Widgets/I_Objective.SetNewText` (`self.IngredientsCollected`)))

(event `/Game/UI/Widgets/I_Objective.SetNewText`
  (params (Text :type Text))
  (bind _returnvalue (`KismetTextLibrary.EqualEqual_TextText` Text (`self.OneTimeUseText`)))
  (if _returnvalue
    (if (`self.1Used?`)
      (set `self.1Used?` _returnvalue)))
  (`KismetSystemLibrary.K2_ClearAndInvalidateTimerHandle` (`self.Dissapear Timer`))
  (`self.NewVoiceLine` Text)
  (`KismetSystemLibrary.Delay` 0.05)
  (`Widget.SetVisibility` (`self.WBP Aliens Talking`) "Visible"))

(event `/Game/UI/Widgets/I_Objective.FinishedText`
  (bind _returnvalue (`KismetSystemLibrary.K2_SetTimerDelegate` (delegate `Dissapear Text`) 7.0))
  (set `self.Dissapear Timer` _returnvalue))

(event `Dissapear Text`
  (`Widget.SetVisibility` (`self.WBP Aliens Talking`) "Hidden"))

(fn `UserConstructionScript`)