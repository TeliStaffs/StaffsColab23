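; Conveyor belt that turns the player's captured ingredients into cooked ingredient actors once the recipe from BP_Till is fulfilled.
; GetIngredient counts down the recipe, and a button press runs CheckInventory before starting the belt once.
; Looping timers spawn each inventory entry with its type, perfection and mesh, and impulse overlapping characters along the belt.
; Widgets show the remaining count, and the final spawn tick fires SpeakToMe and stops the belt.
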(event `self.ReceiveBeginPlay`
  ;[0.5 0.7 1] Set Up wisgets and recipe
  (bind _returnvalue (`GameplayStatics.GetActorOfClass` "/Game/Scripting/Blueprints/Till/BP_Till.BP_Till_C"))
  (add `/Game/Scripting/Blueprints/Till/BP_Till.SetRecipe` _returnvalue (delegate `Set Up`)))

(event `Set Up`
  ;[0.5 0.7 1] Set Up wisgets and recipe
  (set `self.Recipe` (`/Game/Scripting/Blueprints/Till/BP_Till.Recipe` (stale `self.ReceiveBeginPlay` _returnvalue)))
  (bind _aswbp_conveyor_belt (cast `/Game/UI/Widgets/WBP_ConveyorBelt` (`WidgetComponent.GetUserWidgetObject` (`self.IngredientsStoredWidget`))))
  (bind _output_get (set `self.As WBP Conveyor Belt` _aswbp_conveyor_belt))
  (`/Game/UI/Widgets/WBP_ConveyorBelt.UpdateIngredients` _output_get 0)
  (bind _aswbp_conveyor_belt_2 (cast `/Game/UI/Widgets/WBP_ConveyorBelt` (`WidgetComponent.GetUserWidgetObject` (`self.IngredientsStoredWidget1`))))
  (set `self.As WBP Conveyor Belt_0` _aswbp_conveyor_belt_2)
  ;[1 0 0] Must have conveyor button in scene
  (add `/Game/Scripting/Blueprints/ConveyorBelt/BP_Button.StartConveyer` (`self.Button`) (delegate `Start`)))

(event `GetIngredient`
  (params (IngredientType :type "/Game/Scripting/Blueprints/Enemys/Enums/E_IngredientType Enum" :default "NewEnumerator0"))
  (bind _recipe (`self.Recipe`))
  ;[0.5 0.7 1] The same as in the WBP Recipe, tick off ingredients as they are captured, when you have at least the correct amount of each, the conveyor belt can be used
  (bind _keys (`BlueprintMapLibrary.Map_Keys` _recipe))
  (for (_array_element _array_index) _keys
    (if (`|EnumEquality` _array_element IngredientType)
      (bind _values (`BlueprintMapLibrary.Map_Values` (`self.Recipe`)))
      (bind _output (`|GetArrayItem` _values _array_index))
      (if (> _output 0)
        (`BlueprintMapLibrary.Map_Add` _recipe _array_element (- _output 1))))))

(event `Start`
  ;[0.5 0.7 1] If at least one ingredient has been captured, loop through map and spawn ingredients. Once spawned, send them the information they need to give a score if they get cooked
  (bind _allingredients (`self.CheckInventory`))
  (if _allingredients
    (`GameplayStatics.GetActorOfClass` "/Game/Scripting/Blueprints/FoodAssembler/BP_FoodAssembler.BP_FoodAssembler_C")
    (bind _returnvalue (`GameplayStatics.GetActorOfClass` "/Game/Scripting/Blueprints/Character/BP_FirstPersonCharacter.BP_FirstPersonCharacter_C"))
    (bind _returnvalue_2 (`BlueprintMapLibrary.Map_Length` (`/Game/Scripting/Blueprints/Character/AC_Inventory.CapturedIngredients` (`self.GetComponentByClass` _returnvalue "/Game/Scripting/Blueprints/Character/AC_Inventory.AC_Inventory_C"))))
    (if (>= _returnvalue_2 1)
      (`/Engine/EditorBlueprintResources/StandardMacros.DoOnce` false
        (:`Completed`
          (bind _output_get (set `self.IngredientAmount` _returnvalue_2))
          (`/Engine/EditorBlueprintResources/StandardMacros.DecrementInt` _output_get
            (:`  `
              (`self.SpawnIngredients`)
              (bind _returnvalue_3 (`KismetSystemLibrary.K2_SetTimerDelegate` (delegate `SpawnIngredients`) (`self.SpawnDelay`) true))
              (set `self.Spawn Timer` _returnvalue_3)
              (bind _returnvalue_4 (`KismetSystemLibrary.K2_SetTimerDelegate` (delegate `Push Ingredients`) 0.01 true))
              (set `self.Conveyor Belt Timer` _returnvalue_4)
              (`PrimitiveComponent.SetMaterial` (`/Game/Scripting/Blueprints/ConveyorBelt/BP_Button.StaticMesh` (`self.Button`)) 2 "/Game/Materials/M_GlowStandard.M_GlowStandard"))))))))

(event `Push Ingredients`
  ;[0.5 0.7 1] If at least one ingredient has been captured, loop through map and spawn ingredients. Once spawned, send them the information they need to give a score if they get cooked
  ;[0.5 0.7 1] Move object across conveyor belt
  (for _array_element (`PrimitiveComponent.GetOverlappingActors` (`self.PushBox`) null)
    (bind _returnvalue (`self.GetComponentByClass` _array_element "/Script/Engine.CharacterMovementComponent"))
    ;;[0.9893 1 0] Check is valid
    (`/Engine/EditorBlueprintResources/StandardMacros.IsValid` _returnvalue
      (:`Is Valid`
        (`CharacterMovementComponent.AddImpulse` _returnvalue (* (`KismetMathLibrary.Conv_RotatorToVector` (`SceneComponent.K2_GetComponentRotation` (`self.DefaultSceneRoot`))) (`self.ConveyorBeltForce`)) true)))))

(event `SpawnIngredients`
  (bind _ingredientamount (`self.IngredientAmount`))
  ;[0.5 0.7 1] If at least one ingredient has been captured, loop through map and spawn ingredients. Once spawned, send them the information they need to give a score if they get cooked
  (if (< _ingredientamount 0)
    (`self.SpeakToMe`)
    (`KismetSystemLibrary.K2_ClearAndInvalidateTimerHandle` (`self.Spawn Timer`))
    (`KismetSystemLibrary.Delay` 3.0)
    (`KismetSystemLibrary.K2_ClearAndInvalidateTimerHandle` (`self.Conveyor Belt Timer`))
    (`PrimitiveComponent.SetMaterial` (`/Game/Scripting/Blueprints/ConveyorBelt/BP_Button.StaticMesh` (`self.Button`)) 2 "/Game/Materials/HubMaterials/Material__74.Material__74")
    (else
      (`/Game/UI/Widgets/WBP_ConveyorBelt.UpdateIngredients` (`self.As WBP Conveyor Belt`) _ingredientamount)
      (`/Game/UI/Widgets/WBP_ConveyorBelt.UpdateIngredients` (`self.As WBP Conveyor Belt_0`) _ingredientamount)
      (bind _values (`BlueprintMapLibrary.Map_Values` (`/Game/Scripting/Blueprints/Character/AC_Inventory.CapturedIngredients` (`self.GetComponentByClass` (stale `Start` _returnvalue) "/Game/Scripting/Blueprints/Character/AC_Inventory.AC_Inventory_C"))))
      (bind _returnvalue (`|SpawnActorFromClass` "/Game/Scripting/Blueprints/Enemys/BP_CookedEnemyIngredient.BP_CookedEnemyIngredient_C" (`KismetMathLibrary.MakeTransform` (`SceneComponent.K2_GetComponentLocation` (`self.SpawnLocation`))) "Undefined" "OverrideRootScale" null null))
      (bind (_ingredienttype _perfectionlevel _skmesh) (break `/Game/Scripting/Blueprints/Character/F_CapturedEnemyStats` (`|GetArrayItem` _values (`self.IngredientAmount`))))
      (`/Game/Scripting/Blueprints/Enemys/BP_CookedEnemyIngredient.AddStats` _returnvalue _ingredienttype _perfectionlevel _skmesh)
      (`/Engine/EditorBlueprintResources/StandardMacros.DecrementInt` (`self.IngredientAmount`)))))

(fn `CheckInventory`
  (returns (AllIngredients :type Boolean))
  (locals (IngredientCheck :type Boolean))
  ;[0.5 0.7 1] Loop through recipe values, if there is at least one of an ingredient remaining, ingredient check is set to false. If no ingredients are needed, set to true.
  (bind _values (`BlueprintMapLibrary.Map_Values` (`self.Recipe`)))
  (for _array_element _values
    (if (!= _array_element 0)
      (set `local.IngredientCheck` false)
      (break)
      (else
        (set `local.IngredientCheck` true))))
  (return (`local.IngredientCheck`)))

(fn `UserConstructionScript`)