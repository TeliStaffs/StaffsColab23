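; Tutorial teleporter that moves the first-person player to a linked destination teleporter when they overlap its box.
; Non-hub teleporters also require collected ingredients; a game mode hub-activation event can re-enable resettable ones and set that flag.
; Triggering plays Niagara effects, disables the destination and freezes movement until a timer moves the player, plays sound and restores walking.
; The construction script yaws an arrow, and the destination's arrow sets the player's facing on arrival.
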(event `self.ReceiveBeginPlay`
  (bind _asbp_first_person_character (cast `/Game/Scripting/Blueprints/Character/BP_FirstPersonCharacter` (`GameplayStatics.GetPlayerCharacter` 0)))
  (set `self.Player` _asbp_first_person_character)
  (bind _asbp_first_person_game_mode (cast `/Game/Scripting/Blueprints/GameMode/BP_FirstPersonGameMode` (`GameplayStatics.GetGameMode`)))
  (bind _output_get (set `self.As BP First Person Game Mode` _asbp_first_person_game_mode))
  (add `/Game/Scripting/Blueprints/GameMode/BP_FirstPersonGameMode.ActivateHUB` _output_get (delegate `CE_Reset1`)))

(event `CE_Reset1`
  (params (Result :type Boolean))
  (if (`self.WillReset`)
    (set `self.CanTeleport` true)
    (set `self.IngredientsCollected` true)))

(event `self.BoxCollider.OnComponentBeginOverlap`
  (params (OverlappedComponent :type "PrimitiveComponent Object Reference") (OtherActor :type "Actor Object Reference") (OtherComp :type "PrimitiveComponent Object Reference") (OtherBodyIndex :type Integer) (bFromSweep :type Boolean) (SweepResult :type "HitResult Structure (by ref)"))
  ;[1 0.7892 0] Logic Checks
  (cast `/Game/Scripting/Blueprints/Character/BP_FirstPersonCharacter` OtherActor)
  (if (`self.CanTeleport`)
    (if (`self.IsHub?`)
      ;[1 0.7892 0] Activate niagara effects and disable destination teleporter
      (`ActorComponent.Activate` (`self.Niagara`) false :!label _label)
      (set `/Game/Scripting/Blueprints/Teleportation/BP_TutorialTeleporter.CanTeleport` false (`self.TeleporterDestination`))
      (`KismetSystemLibrary.K2_SetTimerDelegate` (delegate `CE_Thing`) 3.0)
      ;[1 0.7892 0] Disable Movement
      (`CharacterMovementComponent.DisableMovement` (`Character.CharacterMovement` (`self.Player`)))
      (`self.CE_StartTeleport`)
      (elif (`self.IngredientsCollected`)
        (goto _label)))))

(event `CE_Thing`
  ;[1 0.7892 0] Activate niagara effects and disable destination teleporter
  (`ActorComponent.Deactivate` (`self.Niagara`)))

(event `CE_StartTeleport`
  (`KismetSystemLibrary.K2_SetTimerDelegate` (delegate `Teleport`) 1.1))

(event `Teleport`
  (bind _teleporterdestination (`self.TeleporterDestination`))
  (bind (_returnvalue_x _returnvalue_y _returnvalue_z) (`KismetMathLibrary.BreakVector` (`self.K2_GetActorLocation` _teleporterdestination)))
  (`self.K2_SetActorLocation` (`self.Player`) (`KismetMathLibrary.MakeVector` _returnvalue_x _returnvalue_y (+ _returnvalue_z 100.0)) false true)
  (`Controller.SetControlRotation` (`GameplayStatics.GetPlayerController` 0) (`SceneComponent.K2_GetComponentRotation` (`self.GetComponentByClass` _teleporterdestination "/Script/Engine.ArrowComponent")))
  (`GameplayStatics.PlaySoundAtLocation` "/Game/Audio/SoundEffects/Teleporter/TeleporterSound.TeleporterSound" (`self.K2_GetActorLocation`) (struct) 1.0 1.0 0.0 null null null null)
  (`CharacterMovementComponent.SetMovementMode` (`Character.CharacterMovement` (`self.Player`)) "MOVE_Walking" 0))

(fn `UserConstructionScript`
  (`SceneComponent.K2_SetWorldRotation` (`self.Arrow`) (`KismetMathLibrary.MakeRotator` 0.0 0.0 (`self.TeleportRotation`)) false false))