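; BP_Till is an interactable till that starts the order by picking the player's recipe, which also allows the teleporters to become functional.
; On first interaction only, it has the alien voice manager tell the player to use the teleporter and picks a random DT_Recipes row.
; It adds that recipe to the player HUD, stores it, and calls SetRecipe to notify other Blueprints.
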(event `self.ReceiveBeginPlay`
  ;[1 0.7892 0] Alien Voice Manager
  (bind _returnvalue (`GameplayStatics.GetActorOfClass` "/Game/Scripting/Blueprints/TutorialLevel/BP_AlienVoiceManager.BP_AlienVoiceManager_C"))
  (`/Engine/EditorBlueprintResources/StandardMacros.IsValid` _returnvalue
    (:`Is Valid`
      (set `self.AVM` _returnvalue))))

(event `/Game/Scripting/Blueprints/ConveyorBelt/BPI_Interact.Interact`
  (bind _avm (`self.AVM`))
  ;[0.5 0.7 1] Will Set the recipe and send a message to other blueprints, telling them to set the recipe, will also allow teleporters to become functional
  (`/Engine/EditorBlueprintResources/StandardMacros.DoOnce` false
    (:`Completed`
      ;;[1 0.7892 0] Alien VoiceManager
      (`/Engine/EditorBlueprintResources/StandardMacros.IsValid` _avm
        (:`Is Valid`
          (`/Game/UI/Widgets/I_Objective.SetNewText` _avm "Now human, go step on my teleporter or else."))
        (:`Is Not Valid`
          _))
      (bind _asbp_first_person_character (cast `/Game/Scripting/Blueprints/Character/BP_FirstPersonCharacter` (`GameplayStatics.GetPlayerCharacter` 0)))
      (set `self.Player HUD` (`/Game/Scripting/Blueprints/Character/BP_FirstPersonCharacter.PlayerHUD` _asbp_first_person_character))
      (bind _outrownames (`DataTableFunctionLibrary.GetDataTableRowNames` "/Game/Scripting/Blueprints/Recipes/DT_Recipes.DT_Recipes"))
      (bind _output_get (set `self.RecipeName` (`KismetArrayLibrary.Array_Random` _outrownames)))
      (`/Game/UI/Widgets/WBP_Recipe.Add Recipe` (`/Game/UI/Widgets/WBP_HUD.WBP_Recipe` (`self.Player HUD`)) _output_get)
      (bind _returnvalue (`|GetDataTableRow` "/Game/Scripting/Blueprints/Recipes/DT_Recipes.DT_Recipes" (`self.RecipeName`))
        (:`then`
          (set `self.Recipe` (`.Recipe_8_90B99CC045854F32ABB1DC81A9D7A2BF` (break `/Game/Scripting/Blueprints/Recipes/F_Recipe` _returnvalue)))
          (`self.SetRecipe`))))))

(fn `UserConstructionScript`)