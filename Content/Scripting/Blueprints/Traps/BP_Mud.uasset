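; BP_Mud is a trap that halves movement speed and jump for actors with an AC_Movement component while they overlap its sphere.
; It also halves the first-person character's dash speed and distance, using a flag on the character to prevent stacking.
; On exit, it scans every BP_Mud's overlap list and only removes the penalties and restores the dash when no other mud still contains that actor.
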(event `self.Sphere.OnComponentBeginOverlap`
  (params (OverlappedComponent :type "PrimitiveComponent Object Reference") (OtherActor :type "Actor Object Reference") (OtherComp :type "PrimitiveComponent Object Reference") (OtherBodyIndex :type Integer) (bFromSweep :type Boolean) (SweepResult :type "HitResult Structure (by ref)"))
  (bind _returnvalue (`self.GetComponentByClass` OtherActor "/Game/Scripting/Blueprints/Character/AC_Movement.AC_Movement_C"))
  (bind _as_bp_first_person_character (`self.As BP First Person Character`))
  ;[1 0.7219 0] Begin Overlap
  (`/Engine/EditorBlueprintResources/StandardMacros.IsValid` _returnvalue
    (:`Is Valid`
      (`KismetArrayLibrary.Array_AddUnique` (`self.OverlappedEntitys`) OtherActor)
      (`/Game/Scripting/Blueprints/Character/AC_Movement.CE_ModifySpeed` _returnvalue 0.5 0.0 "NewEnumerator0")
      (`/Game/Scripting/Blueprints/Character/AC_Movement.CE_Modify Jump` _returnvalue 0.5 0.0 "NewEnumerator0")
      (bind _asbp_first_person_character (cast `/Game/Scripting/Blueprints/Character/BP_FirstPersonCharacter` OtherActor))
      (bind _output_get (set `self.As BP First Person Character` _asbp_first_person_character))
      (if (not (`/Game/Scripting/Blueprints/Character/BP_FirstPersonCharacter.DashAlrAltered` _asbp_first_person_character))
        (set `/Game/Scripting/Blueprints/Character/BP_FirstPersonCharacter.DashAlrAltered` true _output_get)
        (`/Game/Scripting/Blueprints/Character/BP_FirstPersonCharacter.SetDashVariables` _as_bp_first_person_character (* (`/Game/Scripting/Blueprints/Character/BP_FirstPersonCharacter.DashSpeed` _as_bp_first_person_character) 0.5) (* (`/Game/Scripting/Blueprints/Character/BP_FirstPersonCharacter.DashDistance` _as_bp_first_person_character) 0.5))))))

(event `self.Sphere.OnComponentEndOverlap`
  (params (OverlappedComponent :type "PrimitiveComponent Object Reference") (OtherActor :type "Actor Object Reference") (OtherComp :type "PrimitiveComponent Object Reference") (OtherBodyIndex :type Integer))
  (bind _returnvalue (`self.GetComponentByClass` OtherActor "/Game/Scripting/Blueprints/Character/AC_Movement.AC_Movement_C"))
  (bind _as_bp_first_person_character (`self.As BP First Person Character`))
  ;[1 0.7219 0] EndOverlap
  (`KismetArrayLibrary.Array_RemoveItem` (`self.OverlappedEntitys`) OtherActor)
  (set `self.IsStillMuddied` false)
  (`self.CE_IsMuddied`)
  (if (not (`self.IsStillMuddied`))
    (`/Engine/EditorBlueprintResources/StandardMacros.IsValid` _returnvalue
      (:`Is Valid`
        (`/Game/Scripting/Blueprints/Character/AC_Movement.CE_RemoveSlowType` _returnvalue "NewEnumerator0")
        (`/Game/Scripting/Blueprints/Character/AC_Movement.CE_RemoveJForceType` _returnvalue "NewEnumerator0")
        (`/Engine/EditorBlueprintResources/StandardMacros.IsValid` _as_bp_first_person_character
          (:`Is Valid`
            (`/Game/Scripting/Blueprints/Character/BP_FirstPersonCharacter.SetDashVariables` _as_bp_first_person_character (* (`/Game/Scripting/Blueprints/Character/BP_FirstPersonCharacter.DashSpeed` _as_bp_first_person_character) 2.0) (* (`/Game/Scripting/Blueprints/Character/BP_FirstPersonCharacter.DashDistance` _as_bp_first_person_character) 2.0))
            (set `/Game/Scripting/Blueprints/Character/BP_FirstPersonCharacter.DashAlrAltered` false _as_bp_first_person_character)))))))

(event `CE_IsMuddied`
  ;[1 0.7219 0] ChecksIfCharacter is in any other muds
  (bind _outactors (`GameplayStatics.GetAllActorsOfClass` "BP_Mud_C"))
  (for _array_element _outactors
    (if (`KismetArrayLibrary.Array_Contains` (`/Game/Scripting/Blueprints/Traps/BP_Mud.OverlappedEntitys` _array_element) (stale `self.Sphere.OnComponentEndOverlap` OtherActor))
      (set `self.IsStillMuddied` true))))

(fn `UserConstructionScript`)