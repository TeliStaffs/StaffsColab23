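; Actor component that manages temporary slow and speed-up effects on its owning character's walk speed.
; It caches the starting MaxWalkSpeed, then scales it by one minus the summed Environment, Weapon and Damage modifiers, clamped between a floor and ceiling.
; Designer-facing events set or remove a modifier by type.
; Each type has its own timer for resetting it, and reapplying replaces that type's value and restarts its timer.
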(event `CE_ChangePlayerSpeed`
  ;[1 0.7219 0] Sets the characters speed
  (set `CharacterMovementComponent.MaxWalkSpeed` (* (`self.Max Character Speed`) (`KismetMathLibrary.FClamp` (- 1.0 (+ (`self.WeapSlow`) (`self.EnvSlow`) (`self.DmgSlow`))) 0.25 2.0)) (`self.CharacterMovementReference`)))

(event `self.ReceiveBeginPlay`
  ;[1 0.7219 0] Initialise
  (bind _output_get (set `self.CharacterMovementReference` (`Actor.GetComponentByClass` (`self.GetOwner`) "/Script/Engine.CharacterMovementComponent")))
  (bind _output_get_2 (set `self.Max Character Speed` (`CharacterMovementComponent.MaxWalkSpeed` _output_get)))
  (set `self.CurrentMovementSpeed` _output_get_2))

(event `CE_RemoveSlowType`
  (params (SlowType :type "/Game/Scripting/Blueprints/Character/E_SlowTypes Enum" :default "NewEnumerator0"))
  ;[1 0.7219 0] For other bps to specifically remove a slow effect
  ;;[1 1 1] Designers use this
  (switch `/Game/Scripting/Blueprints/Character/E_SlowTypes` SlowType
    (:`NewEnumerator0`
      (`self.CE_Remove Environment Slow`))
    (:`NewEnumerator1`
      (`self.CE_Remove Weapon Slow`))
    (:`NewEnumerator2`
      (`self.CE_Remove Dmg Slow`))))

(event `CE_ModifySpeed`
  (params (`Slowdown %` :type "Float (double-precision)") (SlowdownTime :type "Float (double-precision)") (`Slow Type` :type "/Game/Scripting/Blueprints/Character/E_SlowTypes Enum" :default "NewEnumerator0"))
  (bind _environmentslow (`self.EnvironmentSlow`))
  (bind _weaponslow (`self.WeaponSlow`))
  (bind _damage_slow (`self.Damage Slow`))
  (bind _slowdown__ (`self.Slowdown %`))
  ;[1 0.7219 0] Main modification of speed. Use +or- percentages to modify (IE 0.2 will slow the character 20% and -0.2 will speed up the character 20%)
  ;;[1 1 1] Designers use this
  (set `self.Slowdown Time` SlowdownTime)
  (set `self.Slowdown %` `Slowdown %`)
  (switch `/Game/Scripting/Blueprints/Character/E_SlowTypes` `Slow Type`
    (:`NewEnumerator0`
      (set `self.EnvSlow` _slowdown__)
      (`self.CE_ChangePlayerSpeed`)
      (if (`KismetSystemLibrary.K2_IsValidTimerHandle` _environmentslow)
        (`KismetSystemLibrary.K2_ClearAndInvalidateTimerHandle` _environmentslow))
      (bind _returnvalue (`KismetSystemLibrary.K2_SetTimerDelegate` (`|CreateDelegate` :!event `CE_Remove Environment Slow`) (`self.Slowdown Time`)))
      (set `self.EnvironmentSlow` _returnvalue))
    (:`NewEnumerator1`
      (set `self.WeapSlow` _slowdown__)
      (`self.CE_ChangePlayerSpeed`)
      (if (`KismetSystemLibrary.K2_IsValidTimerHandle` _weaponslow)
        (`KismetSystemLibrary.K2_ClearAndInvalidateTimerHandle` _weaponslow))
      (bind _returnvalue_2 (`KismetSystemLibrary.K2_SetTimerDelegate` (`|CreateDelegate` :!event `CE_Remove Weapon Slow`) (`self.Slowdown Time`)))
      (set `self.WeaponSlow` _returnvalue_2))
    (:`NewEnumerator2`
      (set `self.DmgSlow` _slowdown__)
      (`self.CE_ChangePlayerSpeed`)
      (if (`KismetSystemLibrary.K2_IsValidTimerHandle` _damage_slow)
        (`KismetSystemLibrary.K2_ClearAndInvalidateTimerHandle` _damage_slow))
      (bind _returnvalue_3 (`KismetSystemLibrary.K2_SetTimerDelegate` (`|CreateDelegate` :!event `CE_Remove Environment Slow`) (`self.Slowdown Time`)))
      (set `self.Damage Slow` _returnvalue_3))))

(event `CE_Remove Environment Slow`
  ;[1 0.7219 0] Allows Timers to reset specific slows
  (set `self.EnvSlow` 0.0)
  (`self.CE_ChangePlayerSpeed` :!label _label))

(event `CE_Remove Weapon Slow`
  ;[1 0.7219 0] Allows Timers to reset specific slows
  (set `self.WeapSlow` 0.0)
  (goto _label))

(event `CE_Remove Dmg Slow`
  ;[1 0.7219 0] Allows Timers to reset specific slows
  (set `self.DmgSlow` 0.0)
  (goto _label))