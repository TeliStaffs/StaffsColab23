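; Actor component that serves as a basic ingredient inventory for a character, tallying collected items by enemy type.
; The CE_additem event switches on the EnemyType it receives and increments a separate counter for base enemies, steaks, eggs, noodles or potatoes.
; Each branch prints the updated count to the screen for debugging, and the event stores nothing beyond these totals.
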(event `CE_additem`
  (params (EnemyType :type "/Game/Scripting/Blueprints/Enemys/E_EnemyType Enum" :default "NewEnumerator0"))
  ;[1 0.7219 0] Very basic, just keeps track of number of ingredients
  (switch `/Game/Scripting/Blueprints/Enemys/E_EnemyType` EnemyType
    (:`NewEnumerator0`
      (bind _result (`/Engine/EditorBlueprintResources/StandardMacros.IncrementInt` (`self.NumberOfBaseEnemies`))
        (:`  `
          ;[1 0.7219 0] Debugging
          (`KismetSystemLibrary.PrintString` (`KismetStringLibrary.Concat_StrStr` "Number of base enemies: " (`KismetStringLibrary.Conv_IntToString` _result))))))
    (:`NewEnumerator1`
      (bind _result_2 (`/Engine/EditorBlueprintResources/StandardMacros.IncrementInt` (`self.NumberOfSteaks`))
        (:`  `
          (`KismetSystemLibrary.PrintString` (`KismetStringLibrary.Concat_StrStr` "Number of steaks: " (`KismetStringLibrary.Conv_IntToString` _result_2))))))
    (:`NewEnumerator2`
      (bind _result_3 (`/Engine/EditorBlueprintResources/StandardMacros.IncrementInt` (`self.NumberOfEggs`))
        (:`  `
          (`KismetSystemLibrary.PrintString` (`KismetStringLibrary.Concat_StrStr` "Number of eggs: " (`KismetStringLibrary.Conv_IntToString` _result_3))))))
    (:`NewEnumerator3`
      (bind _result_4 (`/Engine/EditorBlueprintResources/StandardMacros.IncrementInt` (`self.NumberOfNoodles`))
        (:`  `
          (`KismetSystemLibrary.PrintString` (`KismetStringLibrary.Concat_StrStr` "Number of noodles: " (`KismetStringLibrary.Conv_IntToString` _result_4))))))
    (:`NewEnumerator4`
      (bind _result_5 (`/Engine/EditorBlueprintResources/StandardMacros.IncrementInt` (`self.NumberOfPotatoes`))
        (:`  `
          (`KismetSystemLibrary.PrintString` (`KismetStringLibrary.Concat_StrStr` "Number of potatoes: " (`KismetStringLibrary.Conv_IntToString` _result_5))))))))