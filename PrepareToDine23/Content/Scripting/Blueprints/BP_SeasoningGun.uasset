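; BP_SeasoningGun is a shotgun-style hitscan weapon that fires salt on primary fire and pepper on secondary.
; Each input selects a blast particle system and damage type, then calls a shared Fire event.
; Fire spawns the effect at the Arrow and runs several multi-line traces within a narrow elliptical cone, spread mainly in pitch.
; Every returned hit receives damage of the selected type.
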(event `self.OnFireProjectile`
  ;[1 1 1] Set Salt or Pepper
  (set `self.System Template` "/Game/FX/PS_SaltBlast.PS_SaltBlast")
  (set `self.DamageType` "/Game/Scripting/Blueprints/DamageTypes/DamageType_Salt.DamageType_Salt_C")
  (`self.Fire` :!label _label))

(event `self.OnSecondaryAction`
  ;[1 1 1] Set Salt or Pepper
  (set `self.System Template` "/Game/FX/PS_PepperBlast.PS_PepperBlast")
  (set `self.DamageType` "/Game/Scripting/Blueprints/DamageTypes/DamageType_Pepper.DamageType_Pepper_C")
  (goto _label))

(event `Fire`
  (bind _arrow (`self.Arrow`))
  (bind _arrow_2 (`self.Arrow`))
  (bind (_returnvalue_roll _returnvalue_pitch _returnvalue_yaw) (`KismetMathLibrary.BreakRotator` (`SceneComponent.K2_GetComponentRotation` _arrow)))
  (bind _returnvalue (`SceneComponent.K2_GetComponentLocation` _arrow_2))
  ;[1 1 1] Fire spread of shots, damage type switches based on primary or secondary shot
  (`NiagaraFunctionLibrary.SpawnSystemAtLocation` (`self.System Template`) (`SceneComponent.K2_GetComponentLocation` _arrow) (`KismetMathLibrary.MakeRotator` _returnvalue_roll (+ _returnvalue_pitch 270.0) _returnvalue_yaw))
  (for _ (range (`self.ShotsPerFire`))
    (bind _outhits (`KismetSystemLibrary.LineTraceMulti` _returnvalue (+ _returnvalue (* (`KismetMathLibrary.RandomUnitVectorInEllipticalConeInDegrees` (`KismetMathLibrary.Conv_RotatorToVector` (`SceneComponent.K2_GetComponentRotation` _arrow_2)) 1.0 (`self.FireSpread`)) 1000.0)) "TraceTypeQuery1"))
    (for _array_element _outhits
      (`GameplayStatics.ApplyDamage` (`.HitActor` (`GameplayStatics.BreakHitResult` _array_element)) (`self.Base Damage`) null self (`self.DamageType`)))))

(fn `UserConstructionScript`
  (`parent.UserConstructionScript`))