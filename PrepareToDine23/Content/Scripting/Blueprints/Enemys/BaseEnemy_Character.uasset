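; Base enemy character that pairs an AI controller blackboard with a state-based movement setup.
; On BeginPlay it initializes the blackboard and calls StateChange, which writes the state enum to it and sets walk speed, zero for stationary states.
; Damage sets the state to Flee and starts a timer back to Wander, without calling StateChange here.
; The construction script applies default speed and friction from Movement settings.
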(event `self.ReceiveBeginPlay`
  ;[0.2708 0 0.002417] Init
  (bind _asbp_ai_controller (cast `/Game/Scripting/Blueprints/Enemys/AI/BP_AI_Controller` (`self.GetController`)))
  (bind _output_get (set `self.AIController` _asbp_ai_controller))
  (bind _blackboardcomponent (`AIController.UseBlackboard` _output_get (`self.Blackboard Asset`)))
  (set `self.Blackboard Component` _blackboardcomponent)
  (`self.StateChange`))

(event `self.ReceiveAnyDamage`
  (params (Damage :type "Float (single-precision)") (DamageType :type "DamageType Object Reference") (InstigatedBy :type "Controller Object Reference") (DamageCauser :type "Actor Object Reference"))
  (`KismetSystemLibrary.K2_SetTimerDelegate` (delegate `ResumeWander`) 5.0)
  (set `self.State` "NewEnumerator1"))

(event `ResumeWander`
  (set `self.State` "NewEnumerator0"))

(event `StateChange`
  (bind _blackboard_component (`self.Blackboard Component`))
  (bind _state (`self.State`))
  (bind _charactermovement (`self.CharacterMovement`))
  (bind (_movement_maxspeed _movement_friction _movement_wanderspeed _movement_fleespeed _movement_woundedspeed _movement_seekspeed) (break `/Game/Scripting/Blueprints/Enemys/F_AIMovement` (`self.Movement`)))
  ;[0.2708 0 0.002417] on state change
  (switch `/Game/Scripting/Blueprints/Enemys/Enums/E_EnemyStates` (`self.State`)
    (:`NewEnumerator0`
      ;[0.2708 0 0.002417] Update AI BB
      (`BlackboardComponent.SetValueAsEnum` _blackboard_component "States" _state)
      ;[0.2708 0 0.002417] Update Movement
      (set `CharacterMovementComponent.MaxWalkSpeed` _movement_wanderspeed _charactermovement))
    (:`NewEnumerator1`
      (`BlackboardComponent.SetValueAsEnum` _blackboard_component "States" _state)
      (set `CharacterMovementComponent.MaxWalkSpeed` _movement_fleespeed _charactermovement))
    (:`NewEnumerator2`
      (`BlackboardComponent.SetValueAsEnum` _blackboard_component "States" _state)
      (set `CharacterMovementComponent.MaxWalkSpeed` _movement_seekspeed _charactermovement))
    (:`NewEnumerator3`
      (`BlackboardComponent.SetValueAsEnum` _blackboard_component "States" _state)
      (set `CharacterMovementComponent.MaxWalkSpeed` 0.0 _charactermovement))
    (:`NewEnumerator4`
      (`BlackboardComponent.SetValueAsEnum` _blackboard_component "States" _state)
      (set `CharacterMovementComponent.MaxWalkSpeed` 0.0 _charactermovement))
    (:`NewEnumerator5`
      (`BlackboardComponent.SetValueAsEnum` _blackboard_component "States" _state)
      (set `CharacterMovementComponent.MaxWalkSpeed` 0.0 _charactermovement))))

(fn `UserConstructionScript`
  (bind (_movement_maxspeed _movement_friction) (break `/Game/Scripting/Blueprints/Enemys/F_AIMovement` (`self.Movement`)))
  (bind _charactermovement (`self.CharacterMovement`))
  (set `CharacterMovementComponent.MaxWalkSpeed` _movement_maxspeed _charactermovement)
  (set `CharacterMovementComponent.GroundFriction` _movement_friction _charactermovement))