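; Speed pickup that temporarily multiplies the player character's max walk speed.
; Any overlap with its sphere saves the current speed and applies the multiplier to the stored player reference, without checking the overlapping actor.
; After the pickup duration, it restores the saved speed and destroys itself.
; The pickup stays active during the delay, so another overlap overwrites the saved speed and multiplies again.
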(event `self.Sphere1.OnComponentBeginOverlap`
  (params (OverlappedComponent :type "PrimitiveComponent Object Reference") (OtherActor :type "Actor Object Reference") (OtherComp :type "PrimitiveComponent Object Reference") (OtherBodyIndex :type Integer) (bFromSweep :type Boolean) (SweepResult :type "HitResult Structure (by ref)"))
  (bind _charactermovement (`Character.CharacterMovement` (`self.playerRefrence`)))
  (bind _maxwalkspeed (`CharacterMovementComponent.MaxWalkSpeed` _charactermovement))
  ;[1 0 1] Speed Pickup
  (set `self.tmpMaxWalkSpeed` _maxwalkspeed)
  (set `CharacterMovementComponent.MaxWalkSpeed` (* _maxwalkspeed (`self.speedIncrease`)) _charactermovement)
  (`KismetSystemLibrary.Delay` (`self.pickupDuration`))
  (set `CharacterMovementComponent.MaxWalkSpeed` (`self.tmpMaxWalkSpeed`) _charactermovement)
  (`self.K2_DestroyActor`))

(fn `UserConstructionScript`
  (`parent.UserConstructionScript`))