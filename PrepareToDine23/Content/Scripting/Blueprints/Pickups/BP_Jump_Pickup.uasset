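; BP_Jump_Pickup is a pickup that temporarily grants the player a double jump and scales jump height.
; On sphere overlap it calls JustATest, sets NumberOfJumps to two and multiplies the character movement's JumpZVelocity by JumpStrength.
; After a PickupDuration delay, it resets the jump count to one and restores the velocity saved before the boost.
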(event `self.Sphere1.OnComponentBeginOverlap`
  (params (OverlappedComponent :type "PrimitiveComponent Object Reference") (OtherActor :type "Actor Object Reference") (OtherComp :type "PrimitiveComponent Object Reference") (OtherBodyIndex :type Integer) (bFromSweep :type Boolean) (SweepResult :type "HitResult Structure (by ref)"))
  (bind _playerrefrence (`self.playerRefrence`))
  ;[1 0 1] Double Jump Pickup
  (`self.JustATest`)
  (set `/Game/Scripting/Blueprints/Character/BP_FirstPersonCharacter.numberOfJumps` 2 _playerrefrence)
  (bind _output_get (set `self.playerCMRefrence` (`Character.CharacterMovement` _playerrefrence)))
  (bind _jumpzvelocity (`CharacterMovementComponent.JumpZVelocity` _output_get))
  (set `self.tmpJumpZVelocity` _jumpzvelocity)
  (set `CharacterMovementComponent.JumpZVelocity` (* _jumpzvelocity (`self.jumpStrength`)) (`self.playerCMRefrence`))
  (`KismetSystemLibrary.Delay` (`self.pickupDuration`))
  (set `/Game/Scripting/Blueprints/Character/BP_FirstPersonCharacter.numberOfJumps` 1 (`self.playerRefrence`))
  (set `CharacterMovementComponent.JumpZVelocity` (`self.tmpJumpZVelocity`) (`self.playerCMRefrence`)))

(fn `UserConstructionScript`
  (`parent.UserConstructionScript`))