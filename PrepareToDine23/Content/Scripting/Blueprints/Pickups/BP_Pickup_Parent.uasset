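; Base pickup actor that starts a timed pickup when its trigger sphere is overlapped and shows it on screen.
; On overlap it disables collision, hides the visible sphere, plays a sound, stores the player character and fills a WBP_Pickup_Widget from its pickup variables.
; It then calls PickupTriggered with the duration and destroys itself once that time elapses.
; The overlapping actor is never checked; player 0 is always used.
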(event `self.Sphere1.OnComponentBeginOverlap`
  (params (OverlappedComponent :type "PrimitiveComponent Object Reference") (OtherActor :type "Actor Object Reference") (OtherComp :type "PrimitiveComponent Object Reference") (OtherBodyIndex :type Integer) (bFromSweep :type Boolean) (SweepResult :type "HitResult Structure (by ref)"))
  (bind _pickupduration (`self.pickupDuration`))
  (`KismetSystemLibrary.PrintString` "Overlapped")
  (`PrimitiveComponent.SetCollisionEnabled` (`self.Sphere`) "NoCollision")
  (`SceneComponent.SetVisibility` (`self.Sphere`) false false)
  (`PrimitiveComponent.SetCollisionEnabled` (`self.Sphere1`) "NoCollision")
  (`GameplayStatics.PlaySound2D` "/Game/Scripting/FirstPerson/FPWeapon/Audio/FirstPersonTemplateWeaponFire02.FirstPersonTemplateWeaponFire02" 1.0 1.0 0.0 null null)
  (bind _asbp_first_person_character (cast `/Game/Scripting/Blueprints/Character/BP_FirstPersonCharacter` (`GameplayStatics.GetPlayerCharacter` 0)))
  (set `self.fpsCharacterRefrence` _asbp_first_person_character)
  (bind _returnvalue (`|CreateWidget` "/Game/Scripting/Blueprints/Pickups/WBP_Pickup_Widget.WBP_Pickup_Widget_C"))
  (set `/Game/Scripting/Blueprints/Pickups/WBP_Pickup_Widget.PickupImage` (`self.Pickup Image`) _returnvalue)
  (set `/Game/Scripting/Blueprints/Pickups/WBP_Pickup_Widget.pickupNameText` (`self.pickupName`) _returnvalue)
  (set `/Game/Scripting/Blueprints/Pickups/WBP_Pickup_Widget.pickupTimerText` (`self.pickupTimer`) _returnvalue)
  (`UserWidget.AddToViewport` _returnvalue 0)
  (`self.PickupTriggered` _pickupduration)
  (`KismetSystemLibrary.Delay` _pickupduration)
  (`self.K2_DestroyActor`))

(fn `UserConstructionScript`)