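; Child sauce projectile, apparently a cluster piece, that damages and slows characters and leaves sludge on nearby surfaces.
; On overlap, a sphere trace hits each actor with AC_Movement only once and passes other hits to closest-wall selection.
; With a valid wall, it line-traces toward it, spawns BP_SauceSludge at the impact and destroys itself.
; The empty SpawnCluster override prevents infinite recursive spawning; debug traces and prints remain active.
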(event `self.ReceiveBeginPlay`
  (`ProjectileMovementComponent.SetVelocityInLocalSpace` (`self.ProjectileMovement`) (`self.velocity`)))

(event `self.SpawnCluster`
  ;[1 0.7219 0] StopsInfiniteLoop DONOTREMOVE
)

(event `self.CollisionComponent.OnComponentBeginOverlap`
  (params (OverlappedComponent :type "PrimitiveComponent Object Reference") (OtherActor :type "Actor Object Reference") (OtherComp :type "PrimitiveComponent Object Reference") (OtherBodyIndex :type Integer) (bFromSweep :type Boolean) (SweepResult :type "HitResult Structure (by ref)"))
  (bind _returnvalue (`SceneComponent.K2_GetComponentLocation` (`self.CollisionComponent`)))
  ;[1 0.7219 0] MultiSphereTrace
  (`KismetSystemLibrary.PrintString` "Overlapped")
  (bind _outhits (`KismetSystemLibrary.SphereTraceMultiForObjects` :`Start` _returnvalue :`End` _returnvalue :`Radius` (`self.ClusterRadius`) :`ObjectTypes` (`|MakeArray` "ObjectTypeQuery1" "ObjectTypeQuery2" "ObjectTypeQuery3" :!type "EObjectTypeQuery Enum") :`DrawDebugType` "ForDuration" :`DrawTime` 2.0))
  (for _array_element _outhits
    (bind _returnvalue_2 (`self.GetComponentByClass` (`.HitActor` (`GameplayStatics.BreakHitResult` _array_element)) "/Game/Scripting/Blueprints/Character/AC_Movement.AC_Movement_C"))
    ;[1 0.7219 0] ChecksIfCharacterOrEnvironment
    (`/Engine/EditorBlueprintResources/StandardMacros.IsValid` _returnvalue_2
      (:`Is Valid`
        ;[1 0.7219 0] Slowdowns And Damage
        (if (not (`KismetArrayLibrary.Array_Contains` (`self.HitArray`) _returnvalue_2))
          (`/Game/Scripting/Blueprints/Character/AC_Movement.CE_ModifySpeed` _returnvalue_2 0.5 1.2 "NewEnumerator2")
          (`GameplayStatics.ApplyDamage` (`.HitActor` (`GameplayStatics.BreakHitResult` _array_element)) (`self.SauceDamage`) null null "/Game/Scripting/Blueprints/DamageTypes/DamageType_Sauce.DamageType_Sauce_C")
          (`KismetSystemLibrary.PrintString` "Damaging")
          (`KismetArrayLibrary.Array_Add` (`self.HitArray`) _returnvalue_2)))
      (:`Is Not Valid`
        (`self.CE_Wall` null))))
  (`self.CE_SpawnGoop`))

(event `CE_Wall`
  (params (OverlappedActor :type "Actor Object Reference"))
  (bind _closestwall (`self.ClosestWall`))
  ;[1 0.7219 0] CalculatingClosestWall
  (`/Engine/EditorBlueprintResources/StandardMacros.IsValid` _closestwall
    (:`Is Valid`
      (if (< (`self.GetDistanceTo` OverlappedActor) (`self.GetDistanceTo` _closestwall))
        (set `self.ClosestWall` OverlappedActor)))
    (:`Is Not Valid`
      (set `self.ClosestWall` OverlappedActor))))

(event `CE_SpawnGoop`
  (bind _closestwall (`self.ClosestWall`))
  (`/Engine/EditorBlueprintResources/StandardMacros.IsValid` _closestwall
    (:`Is Valid`
      (bind _outhit (`KismetSystemLibrary.LineTraceSingleForObjects` :`Start` (`self.K2_GetActorLocation`) :`End` (`self.K2_GetActorLocation` _closestwall) :`ObjectTypes` (`|MakeArray` "ObjectTypeQuery1" "ObjectTypeQuery2" :!type "EObjectTypeQuery Enum") :`DrawDebugType` "ForDuration"))
      (`|SpawnActorFromClass` "/Game/Scripting/Blueprints/Weapons/BP_SauceSludge.BP_SauceSludge_C" (`KismetMathLibrary.MakeTransform` (`.Location` (`GameplayStatics.BreakHitResult` _outhit))) "Undefined" "OverrideRootScale" null (`self.SauceDamage`) null)
      (`self.K2_DestroyActor`))))

(fn `UserConstructionScript`
  (`parent.UserConstructionScript`))