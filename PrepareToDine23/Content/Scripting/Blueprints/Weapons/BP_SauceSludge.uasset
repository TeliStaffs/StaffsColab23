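; BP_SauceSludge is a sauce hazard zone that slows and damages actors with an AC_Movement component.
; On collision overlap it applies a slowdown and immediate sauce damage, then starts a looping timer, apparently for DamageTick, which damages everything in EnemyArray.
; End overlap removes the slow, but nothing here fills EnemyArray or clears the timer.
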(event `self.Collision.OnComponentBeginOverlap`
  (params (OverlappedComponent :type "PrimitiveComponent Object Reference") (OtherActor :type "Actor Object Reference") (OtherComp :type "PrimitiveComponent Object Reference") (OtherBodyIndex :type Integer) (bFromSweep :type Boolean) (SweepResult :type "HitResult Structure (by ref)"))
  (bind _returnvalue (`self.GetComponentByClass` OtherActor "/Game/Scripting/Blueprints/Character/AC_Movement.AC_Movement_C"))
  (`KismetSystemLibrary.PrintString` "Overlap")
  (`/Engine/EditorBlueprintResources/StandardMacros.IsValid` _returnvalue
    (:`Is Valid`
      (`/Game/Scripting/Blueprints/Character/AC_Movement.CE_ModifySpeed` _returnvalue 0.4 0.0 "NewEnumerator2")
      ;[1 0.7219 0] DamageStuf
      (`GameplayStatics.ApplyDamage` OtherActor (`self.SauceDamage`) null null "/Game/Scripting/Blueprints/DamageTypes/DamageType_Sauce.DamageType_Sauce_C")
      (bind _returnvalue_2 (`KismetSystemLibrary.K2_SetTimerDelegate` (`|CreateDelegate` :!event `DamageTick`) (`self.DamageFrequency`) true))
      (set `self.Damage Tick` _returnvalue_2))))

(event `DamageTick`
  ;[1 0.7219 0] DamageStuf
  (for _array_element (`self.EnemyArray`)
    (`GameplayStatics.ApplyDamage` _array_element (`self.SauceDamage`) null null "/Game/Scripting/Blueprints/DamageTypes/DamageType_Sauce.DamageType_Sauce_C")))

(event `self.Collision.OnComponentEndOverlap`
  (params (OverlappedComponent :type "PrimitiveComponent Object Reference") (OtherActor :type "Actor Object Reference") (OtherComp :type "PrimitiveComponent Object Reference") (OtherBodyIndex :type Integer))
  (`/Game/Scripting/Blueprints/Character/AC_Movement.CE_RemoveSlowType` (`self.GetComponentByClass` OtherActor "/Game/Scripting/Blueprints/Character/AC_Movement.AC_Movement_C") "NewEnumerator2"))

(fn `UserConstructionScript`)