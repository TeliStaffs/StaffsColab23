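; Prototype flamethrower pickup that snaps to the first-person character's grip socket on overlap and binds to its use and release-primary events.
; While firing, a looping timer prints the names of actors tracked by a sphere overlap and adds heat; the flame damage call is disconnected.
; Reaching max overheat blocks firing, and a delayed timer then counts heat down, re-enabling fire at zero.
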(event `self.SphereCollision.OnComponentBeginOverlap`
  (params (OverlappedComponent :type "PrimitiveComponent Object Reference") (OtherActor :type "Actor Object Reference") (OtherComp :type "PrimitiveComponent Object Reference") (OtherBodyIndex :type Integer) (bFromSweep :type Boolean) (SweepResult :type "HitResult Structure (by ref)"))
  (bind _asbp_first_person_character (cast `/Game/Scripting/Blueprints/Character/BP_FirstPersonCharacter` OtherActor)
    (:`then`
      (set `self.FirstPersonCharacterReference` _asbp_first_person_character)
      (`self.K2_AttachToComponent` self (`/Game/Scripting/Blueprints/Character/BP_FirstPersonCharacter.FirstPersonMesh` (`self.FirstPersonCharacterReference`)) "GripPoint" "SnapToTarget" "SnapToTarget" "SnapToTarget" true)
      (add `/Game/Scripting/Blueprints/Character/BP_FirstPersonCharacter.OnUseItem` (`self.FirstPersonCharacterReference`) (`|CreateDelegate` :!event `OnFireProjectile`))
      ;[1 0.7219 0] Bind for stopping the fire
      (add `/Game/Scripting/Blueprints/Character/BP_FirstPersonCharacter.OnReleasePrimary` (`self.FirstPersonCharacterReference`) (`|CreateDelegate` :!event `CE_Stop Fire`)))
    (:`CastFailed`
      (`KismetSystemLibrary.PrintString` "Cast to BP_FirstPersonCharacter FAILED"))))

(event `CE_Stop Fire`
  ;[1 0.7219 0] Stop firing projectiles
  (`KismetSystemLibrary.K2_ClearAndInvalidateTimerHandle` (`self.FiringTimer`)))

(event `self.OnFireProjectile`
  ;[1 0.7219 0] Start Firing projectile
  (if (`self.CanFire?`)
    (bind _returnvalue (`KismetSystemLibrary.K2_SetTimerDelegate` (delegate `CE_FireProj`) 0.05 true))
    (set `self.FiringTimer` _returnvalue)))

(event `CE_FireProj`
  ;[1 0.7219 0] Individual projectile fire
  (for _array_element (`self.Actors`)
    (`KismetSystemLibrary.PrintString` (`KismetSystemLibrary.GetDisplayName` _array_element)))
  (`self.CE_AddOverheat`))

(event `self.Sphere.OnComponentBeginOverlap`
  (params (OverlappedComponent :type "PrimitiveComponent Object Reference") (OtherActor :type "Actor Object Reference") (OtherComp :type "PrimitiveComponent Object Reference") (OtherBodyIndex :type Integer) (bFromSweep :type Boolean) (SweepResult :type "HitResult Structure (by ref)"))
  (`KismetArrayLibrary.Array_Add` (`self.Actors`) OtherActor))

(event `self.Sphere.OnComponentEndOverlap`
  (params (OverlappedComponent :type "PrimitiveComponent Object Reference") (OtherActor :type "Actor Object Reference") (OtherComp :type "PrimitiveComponent Object Reference") (OtherBodyIndex :type Integer))
  (`KismetArrayLibrary.Array_RemoveItem` (`self.Actors`) OtherActor))

(event `CE_AddOverheat`
  (bind _maxoverheat (`self.MaxOverheat`))
  ;[1 0.7219 0] Overheat Flamethrower Logic
  (`KismetSystemLibrary.K2_ClearAndInvalidateTimerHandle` (`self.CoolingTimer`))
  (bind _result (`/Engine/EditorBlueprintResources/StandardMacros.IncrementFloat` (`self.CurrentOverheat`))
    (:`  `
      (`KismetSystemLibrary.PrintString` (`KismetStringLibrary.Concat_StrStr` "Current Overheat: " (`KismetStringLibrary.Conv_DoubleToString` _result) "/" (`KismetStringLibrary.Conv_DoubleToString` _maxoverheat)))
      (if (not (< _result _maxoverheat))
        (set `self.CanFire?` false)
        (`self.CE_Stop Fire`))
      (bind _returnvalue (`KismetSystemLibrary.K2_SetTimerDelegate` (delegate `CE_Cooldown`) (`self.CooldownTime`)))
      (set `self.TimeUntilCool` _returnvalue))))

(event `CE_Cooldown`
  ;[1 0.7219 0] Cooldown Flamethrower
  (bind _returnvalue (`KismetSystemLibrary.K2_SetTimerDelegate` (delegate `CE_IncrementCooldown`) 0.03 true))
  (set `self.CoolingTimer` _returnvalue))

(event `CE_IncrementCooldown`
  ;[1 0.7219 0] Cooldown Flamethrower
  (bind _result (`/Engine/EditorBlueprintResources/StandardMacros.DecrementFloat` (`self.CurrentOverheat`))
    (:`  `
      (`KismetSystemLibrary.PrintString` (`KismetStringLibrary.Conv_DoubleToString` _result))
      (if (== _result 0.0)
        (set `self.CanFire?` true)
        (`KismetSystemLibrary.K2_ClearAndInvalidateTimerHandle` (`self.CoolingTimer`))))))

(fn `UserConstructionScript`
  (`parent.UserConstructionScript`))