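; BP_Melee_Parent is a melee weapon Blueprint, named as a parent class, that swings on primary action input and applies damage on overlap.
; A Swing timeline lerps the root component's rotation from StartRotation, captured from WeaponMesh in the construction script, toward that rotation combined with RotationOffset.
; CollisionBox overlaps apply knife-type damage and call the WeaponCollided dispatcher, with no check for an active swing.
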(event `InputAction|PrimaryAction`
  (params (Key :type "Key Structure"))
  (bind _startrotation (`self.StartRotation`))
  (:`Pressed`
    (`KismetSystemLibrary.PrintString` "Swing")
    (bind (_direction _newtrack_0) (`Timeline|Swing`)
      (:`Update`
        (`SceneComponent.K2_SetRelativeRotation` (`self.DefaultSceneRoot`) (`KismetMathLibrary.RLerp` _startrotation (`KismetMathLibrary.ComposeRotators` _startrotation (`self.RotationOffset`)) _newtrack_0) false false)))))

(event `self.CollisionBox.OnComponentBeginOverlap`
  (params (OverlappedComponent :type "PrimitiveComponent Object Reference") (OtherActor :type "Actor Object Reference") (OtherComp :type "PrimitiveComponent Object Reference") (OtherBodyIndex :type Integer) (bFromSweep :type Boolean) (SweepResult :type "HitResult Structure (by ref)"))
  (`GameplayStatics.ApplyDamage` null (`self.Damage`) null null "/Game/Scripting/Blueprints/DamageTypes/DamageType_Knife.DamageType_Knife_C")
  (`self.WeaponCollided`))

(fn `UserConstructionScript`
  (set `self.StartRotation` (`SceneComponent.RelativeRotation` (`self.WeaponMesh`))))