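; BP_Weapon_Parent is the base Blueprint for weapons, applying each weapon's movement traits to the first-person character.
; On BeginPlay it finds BP_FirstPersonCharacter, passes dash speed and distance to it, and applies the weapon's slowdown through the character's ACMovement component.
; It then calls empty BeginPlayMelee and BeginPlayGuns events, which act as hooks for melee and gun setup.
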(event `self.ReceiveBeginPlay`
  (`KismetSystemLibrary.PrintString` "Swapped")
  (bind _returnvalue (`GameplayStatics.GetActorOfClass` "/Game/Scripting/Blueprints/Character/BP_FirstPersonCharacter.BP_FirstPersonCharacter_C"))
  (`/Game/Scripting/Blueprints/Character/BP_FirstPersonCharacter.SetDashVariables` _returnvalue (`self.DashSpeed`) (`self.DashDistance`))
  ;[1 0.7219 0] Sorry for jacking your bp mike! Do whatever with this aslong as its still called
  (`self.CE_SetWeaponMoveSpeed`)
  (`self.BeginPlayMelee`)
  (`self.BeginPlayGuns`))

(event `BeginPlayMelee`)

(event `BeginPlayGuns`)

(event `CE_SetWeaponMoveSpeed`
  ;[1 0.7219 0] Edits the characters movement speed based on weapon
  (`/Game/Scripting/Blueprints/Character/AC_Movement.CE_ModifySpeed` (`/Game/Scripting/Blueprints/Character/BP_FirstPersonCharacter.AC_Movement` (stale `self.ReceiveBeginPlay` _returnvalue)) (`self.WeaponSlowdown%`) 0.0 "NewEnumerator1"))

(fn `UserConstructionScript`)