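; Prototype flamethrower pickup that snaps to the first-person character's GripPoint on overlap and binds to its use-item events.
; A looping timer spawns BP_FlameProjectile from the Ammo socket along the camera rotation with random spread.
; Each shot adds overheat, cutting fire at the maximum, and restarts a delayed cooldown timer that counts heat down, re-enabling fire at zero.
; Overheat values print to screen.
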(event `self.SphereCollision.OnComponentBeginOverlap`
  (params (OverlappedComponent :type "PrimitiveComponent Object Reference") (OtherActor :type "Actor Object Reference") (OtherComp :type "PrimitiveComponent Object Reference") (OtherBodyIndex :type Integer) (bFromSweep :type Boolean) (SweepResult :type "HitResult Structure (by ref)"))
  (bind _asbp_first_person_character (cast `/Game/FirstPerson/Blueprints/BP_FirstPersonCharacter` OtherActor)
    (:`then`
      (set `self.FirstPersonCharacterReference` _asbp_first_person_character)
      (`self.K2_AttachToComponent` self (`/Game/FirstPerson/Blueprints/BP_FirstPersonCharacter.FirstPersonMesh` (`self.FirstPersonCharacterReference`)) "GripPoint" "SnapToTarget" "SnapToTarget" "SnapToTarget" true)
      (add `/Game/FirstPerson/Blueprints/BP_FirstPersonCharacter.OnUseItem` (`self.FirstPersonCharacterReference`) (`|CreateDelegate` :!event `OnFireProjectile`))
      (add `/Game/FirstPerson/Blueprints/BP_FirstPersonCharacter.OnEndUseItem` (`self.FirstPersonCharacterReference`) (`|CreateDelegate` :!event `CE_Stop Fire`)))
    (:`CastFailed`
      (`KismetSystemLibrary.PrintString` "Cast to BP_FirstPersonCharacter FAILED"))))

(event `CE_Stop Fire`
  (`KismetSystemLibrary.K2_ClearAndInvalidateTimerHandle` (`self.FiringTimer`)))

(event `self.OnFireProjectile`
  (if (`self.CanFire?`)
    (bind _returnvalue (`KismetSystemLibrary.K2_SetTimerDelegate` (delegate `CE_FireProj`) 0.05 true))
    (set `self.FiringTimer` _returnvalue)))

(event `CE_FireProj`
  (bind _returnvalue (`PlayerCameraManager.GetCameraRotation` (`GameplayStatics.GetPlayerCameraManager` 0)))
  (`|SpawnActorFromClass` "/Game/Prototype/BP_FlameProjectile.BP_FlameProjectile_C" (`KismetMathLibrary.MakeTransform` (+ (`SceneComponent.GetSocketLocation` (`self.SkeletalMesh`) "Ammo") (`KismetMathLibrary.GreaterGreater_VectorRotator` (`self.ProjectileOffset`) _returnvalue)) (`KismetMathLibrary.MakeRotator` (+ (.roll _returnvalue) (`KismetMathLibrary.RandomFloatInRange` -2.5 2.5)) (+ (.pitch _returnvalue) (`KismetMathLibrary.RandomFloatInRange` -2.5 2.5)) (+ (.yaw _returnvalue) (`KismetMathLibrary.RandomFloatInRange` -2.5 2.5)))) "Undefined" "OverrideRootScale" null (`self.Flame Damage`) null)
  (`self.CE_AddOverheat`))

(event `CE_AddOverheat`
  (bind _maxoverheat (`self.MaxOverheat`))
  (`KismetSystemLibrary.K2_ClearAndInvalidateTimerHandle` (`self.CoolingTimer`))
  (bind _result (`/Engine/EditorBlueprintResources/StandardMacros.IncrementFloat` (`self.CurrentOverheat`))
    (:`  `
      (`KismetSystemLibrary.PrintString` (`KismetStringLibrary.Concat_StrStr` "Current Overheat: " (`KismetStringLibrary.Conv_DoubleToString` _result) "/" (`KismetStringLibrary.Conv_DoubleToString` _maxoverheat)))
      (if (not (< _result _maxoverheat))
        (set `self.CanFire?` false)
        (`self.CE_Stop Fire`))
      (bind _returnvalue (`KismetSystemLibrary.K2_SetTimerDelegate` (delegate `CE_Cooldown`) (`self.CooldownTime`)))
      (set `self.TimeUntilCool` _returnvalue))))

(event `CE_Cooldown`
  (bind _returnvalue (`KismetSystemLibrary.K2_SetTimerDelegate` (delegate `CE_IncrementCooldown`) 0.03 true))
  (set `self.CoolingTimer` _returnvalue))

(event `CE_IncrementCooldown`
  (bind _result (`/Engine/EditorBlueprintResources/StandardMacros.DecrementFloat` (`self.CurrentOverheat`))
    (:`  `
      (`KismetSystemLibrary.PrintString` (`KismetStringLibrary.Conv_DoubleToString` _result))
      (if (== _result 0.0)
        (set `self.CanFire?` true)
        (`KismetSystemLibrary.K2_ClearAndInvalidateTimerHandle` (`self.CoolingTimer`))))))

(fn `UserConstructionScript`
  (`parent.UserConstructionScript`))