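; Prototype flamethrower weapon that sprays flame projectiles repeatedly while firing.
; OnFireProjectile starts a fast looping timer, and releasing the left mouse button clears it.
; Each tick spawns a BP_FlameProjectile with its damage, offset from the mesh's Ammo socket along camera rotation, and plays the first-person fire montage.
; The firing sound node is disconnected, so it never plays.
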(event `Key|LeftMouseButton`
  (params (Key :type "Key Structure"))
  (:`Released`
    (`KismetSystemLibrary.K2_ClearAndInvalidateTimerHandle` (`self.FiringTimer`))))

(event `self.OnFireProjectile`
  (bind _returnvalue (`KismetSystemLibrary.K2_SetTimerDelegate` (delegate `CE_FireProj`) 0.05 true))
  (set `self.FiringTimer` _returnvalue))

(event `CE_FireProj`
  (bind _returnvalue (`PlayerCameraManager.GetCameraRotation` (`GameplayStatics.GetPlayerCameraManager` 0)))
  (`|SpawnActorFromClass` "/Game/BP_FlameProjectile.BP_FlameProjectile_C" (`KismetMathLibrary.MakeTransform` (+ (`SceneComponent.GetSocketLocation` (`self.SkeletalMesh`) "Ammo") (`KismetMathLibrary.GreaterGreater_VectorRotator` (`self.ProjectileOffset`) _returnvalue)) _returnvalue) "Undefined" "OverrideRootScale" null 3.0 null)
  (`AnimInstance.Montage_Play` (`SkeletalMeshComponent.GetAnimInstance` (`/Game/FirstPerson/Blueprints/BP_FirstPersonCharacter.FirstPersonMesh` (`self.FirstPersonCharacterReference`))) "/Game/FirstPersonArms/Animations/FirstPersonFire_Montage.FirstPersonFire_Montage" 1.0 "MontageLength" 0.0 true))

(fn `UserConstructionScript`
  (`parent.UserConstructionScript`))